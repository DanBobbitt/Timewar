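; HUD for an RTS-style game that draws the mouse drag selection box and name labels over units.
; Each DrawHUD polls the left mouse button, using paired DoOnce gates to capture drag start and end, then passes both corners to MyPlayerController's BoxSelect.
; It also projects every Unit's position to screen and draws its name, highlighted if selected, otherwise colored by ownership.
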(event `self.ReceiveBeginPlay`
  (bind _asmy_player_controller (cast `/Game/Timewar/Blueprints/MyPlayerController` (`self.GetOwningPlayerController`)))
  (set `self.MyPlayerController` _asmy_player_controller))

(event `self.ReceiveDrawHUD`
  (params (SizeX :type Integer) (SizeY :type Integer))
  (`|ExecutionSequence`
    (:`then_0`
      (`self.Selection Box`))
    (:`then_1`
      (`self.Render Unit Icons`))))

(fn `UserConstructionScript`)