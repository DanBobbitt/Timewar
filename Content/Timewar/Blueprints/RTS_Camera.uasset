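; RTS camera pawn for Timewar that moves, pans, rotates and zooms the view, mostly through an InvisiblePoint component.
; Axis inputs drive movement, while gates route mouse motion to Alt rotation (clamped pitch) or middle-mouse actor panning, otherwise to screen-edge scrolling.
; Wheel zoom halves or doubles altitude within limits, scaling the position about the cursor's trace hit.
; Zoom requires TW_PlayerController_Lobby; the ZoomToMousePos helper is unused here.
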(event `self.ReceivePossessed`
  (params (NewController :type "Controller Object Reference"))
  (bind _astw_player_controller_lobby (cast `/Game/Timewar/Blueprints/TW_PlayerController_Lobby` NewController))
  (set `self.OwningController` _astw_player_controller_lobby))

(event `InputAxis|MoveForward`
  (params (AxisValue :type "Float (single-precision)"))
  ;[1 1 1] Camera Movement  + Zoom
  (`self.Camera Move Macro` AxisValue (stale `InputAxis|MoveRight` AxisValue) :!label _label))

(event `Key|MouseScrollUp`
  (params (Key :type "Key Structure"))
  ;[1 1 1] Camera Movement  + Zoom
  (:`Pressed`
    (`self.Camera Zoom Macro` :!label _label_2)))

(event `self.ReceiveUnpossessed`
  (params (OldController :type "Controller Object Reference"))
  (set `self.OwningController` null))

(event `Key|MouseScrollDown`
  (params (Key :type "Key Structure"))
  ;[1 1 1] Camera Movement  + Zoom
  (:`Pressed`
    (goto _label_2 :!via `Zoom Out`)))

(event `InputAxis|MoveRight`
  (params (AxisValue :type "Float (single-precision)"))
  ;[1 1 1] Camera Movement  + Zoom
  (goto _label :!via `Left and Right`))

(event `self.ReceiveBeginPlay`
  (set `PlayerController.bShowMouseCursor` true (`GameplayStatics.GetPlayerController` 0))
  (`SceneComponent.K2_SetWorldLocation` (`self.InvisiblePoint`) (0.0 0.0 2000.0) false false))

(event `Key|LeftAlt`
  (params (Key :type "Key Structure"))
  ;[1 1 1] Rotation, Panning or Screen Edge
  (:`Pressed`
    (set `self.Camera Rotating` true)
    (`|ExecutionSequence`
      (:`then_0`
        (goto _label_3 :!via `Open`))
      (:`then_1`
        (goto _label_8 :!via `Open`))))
  (:`Released`
    (set `self.Camera Rotating` false)
    (`|ExecutionSequence`
      (:`then_0`
        (goto _label_3 :!via `Close`))
      (:`then_1`
        (goto _label_8 :!via `Close`)))))

(event `InputAxisKey|MouseX`
  (params (AxisValue :type "Float (single-precision)"))
  ;[1 1 1] Rotation, Panning or Screen Edge
  (if (xor (`self.Camera Rotating`) (`self.Camera Panning`))
    (if (`self.Camera Rotating`)
      (`/Engine/EditorBlueprintResources/StandardMacros.Gate` true :!label _label_3
        (:`Exit`
          (`self.Camera Rotate Macro` AxisValue (stale `InputAxisKey|MouseY` AxisValue) :!label _label_4)))
      (else
        (`/Engine/EditorBlueprintResources/StandardMacros.Gate` true :!label _label_5
          (:`Exit`
            (`self.Camera Pan Macro` AxisValue (stale `InputAxisKey|MouseY` AxisValue) :!label _label_6)))))
    (else
      (`self.Camera Screenedge Macro` :!label _label_7))))

(event `InputAxisKey|MouseY`
  (params (AxisValue :type "Float (single-precision)"))
  ;[1 1 1] Rotation, Panning or Screen Edge
  (if (xor (`self.Camera Rotating`) (`self.Camera Panning`))
    (if (`self.Camera Rotating`)
      (`/Engine/EditorBlueprintResources/StandardMacros.Gate` true :!label _label_8
        (:`Exit`
          (goto _label_4 :!via `Mouse LeftRight`)))
      (else
        (`/Engine/EditorBlueprintResources/StandardMacros.Gate` true :!label _label_9
          (:`Exit`
            (goto _label_6 :!via `MouseY`)))))
    (else
      (goto _label_7 :!via `ForwardAndBack`))))

(event `Key|MiddleMouseButton`
  (params (Key :type "Key Structure"))
  ;[1 1 1] Rotation, Panning or Screen Edge
  (:`Pressed`
    (set `self.Camera Panning` true)
    (`|ExecutionSequence`
      (:`then_0`
        (goto _label_5 :!via `Open`))
      (:`then_1`
        (goto _label_9 :!via `Open`))))
  (:`Released`
    (set `self.Camera Panning` false)
    (`|ExecutionSequence`
      (:`then_0`
        (goto _label_5 :!via `Close`))
      (:`then_1`
        (goto _label_9 :!via `Close`)))))

(fn `UserConstructionScript`)