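; Base actor for a module within a Unit_Base, holding its own health, equipment and formation offset.
; On BeginPlay it spawns each equipment slot's actor onto a mesh socket with the parent pawn as instigator, then caches the parent unit.
; Each tick it yaws toward its current target, or faces along the unit's velocity without one.
; Radial and point damage subtract truncated amounts from Health, and UpdateDesiredOffset scatters its formation slot within a radius.
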(event `Update Desired Offset`
  (params (`Random X` :type "Float (double-precision)") (`Random Y` :type "Float (double-precision)") (Radius :type "Float (double-precision)"))
  (set `self.(Local) Desired Offset` (+ (`self.(Local) Formation Slot`) (* (`KismetMathLibrary.MakeVector` `Random X` `Random Y`) Radius))))

(event `self.ReceiveRadialDamage`
  (params (DamageReceived :type "Float (single-precision)") (DamageType :type "DamageType Object Reference") (Origin :type "Vector Structure") (HitInfo :type "HitResult Structure (by ref)") (InstigatedBy :type "Controller Object Reference") (DamageCauser :type "Actor Object Reference"))
  (`self.TakeAOEDamage` DamageReceived))

(event `self.ReceivePointDamage`
  (params (Damage :type "Float (single-precision)") (DamageType :type "DamageType Object Reference") (HitLocation :type "Vector Structure") (HitNormal :type "Vector Structure") (HitComponent :type "PrimitiveComponent Object Reference") (BoneName :type Name) (ShotFromDirection :type "Vector Structure") (InstigatedBy :type "Controller Object Reference") (DamageCauser :type "Actor Object Reference") (HitInfo :type "HitResult Structure (by ref)"))
  (`self.TakePointDamage` Damage))

(event `self.ReceiveBeginPlay`
  (`self.SpawnAndAttachEquipment`)
  (bind _asunit_base (cast `/Game/Timewar/Blueprints/Units/Unit_Base` (`self.GetParentActor`)))
  (set `self.ParentUnit` _asunit_base))

(event `self.ReceiveTick`
  (params (DeltaSeconds :type "Float (single-precision)"))
  (bind _defaultsceneroot (`self.DefaultSceneRoot`))
  (bind (_returnvalue_roll _returnvalue_pitch _returnvalue_yaw) (`KismetMathLibrary.BreakRotator` (`KismetMathLibrary.FindLookAtRotation` (`SceneComponent.K2_GetComponentLocation` (`self.DefaultSceneRoot`)) (`self.K2_GetActorLocation` (`self.CurrentTarget`)))))
  (`/Engine/EditorBlueprintResources/StandardMacros.IsValid` (`self.CurrentTarget`)
    (:`Is Valid`
      (`SceneComponent.K2_SetWorldRotation` _defaultsceneroot (`KismetMathLibrary.MakeRotator` 0.0 0.0 _returnvalue_yaw) false false))
    (:`Is Not Valid`
      (`SceneComponent.K2_SetWorldRotation` _defaultsceneroot (`KismetMathLibrary.MakeRotFromX` (`self.GetVelocity` (`self.ParentUnit`))) false false))))

(fn `SpawnAndAttachEquipment`
  (for _array_element (`self.EquipmentSlots`)
    (bind _aspawn (cast `Pawn` (`self.GetParentActor`))
      (:`then`
        (bind _returnvalue (`|SpawnActorFromClass` (break `/Game/Timewar/Blueprints/UnitComponents/EquipmentSlot` _array_element) (`self.GetTransform`) "AlwaysSpawn" "OverrideRootScale" null _aspawn))
        (`self.K2_AttachToComponent` _returnvalue (`self.Mesh`) (`.SocketName_27_AA068AC44829C3BD18A28D8C52975812` (break `/Game/Timewar/Blueprints/UnitComponents/EquipmentSlot` _array_element)) "SnapToTarget" "SnapToTarget" "SnapToTarget" true))
      (:`CastFailed`
        (`KismetSystemLibrary.PrintString` "Module Not child of Pawn! Failed to spawn equipment." true true (struct :`R` 1.0 :`G` 0.025124 :`A` 1.0) 10.0)))))

(fn `TakeAOEDamage`
  (params (`Damage Recieved` :type "Float (double-precision)"))
  (set `self.Health` (- (`self.Health`) (`KismetMathLibrary.FTrunc` `Damage Recieved`))))

(fn `TakePointDamage`
  (params (`Hit Damage` :type "Float (double-precision)"))
  (set `self.Health` (- (`self.Health`) (`KismetMathLibrary.FTrunc` `Hit Damage`))))

(fn `UserConstructionScript`)