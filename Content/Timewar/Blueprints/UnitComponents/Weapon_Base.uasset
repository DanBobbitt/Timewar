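; Base weapon component for units that fires hitscan shots on the server with spread, damage and reloading.
; SetShooting toggles a self-repeating server fire loop paced by TimeBetweenShots.
; Each shot line-traces within an accuracy-derived cone, decrements ammo without checking it, and damages hit actors.
; Muzzle and impact particles are multicast and skipped on dedicated servers; reload refills after a delay and resumes firing if still active.
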(event `Set Shooting`
  (params (Shooting :type Boolean))
  ;[1 1 1] Clientside
  (`self.Set Shooting (Server)` Shooting))

(event `Fire (Server)`
  ;[1 1 1] Firing Shots
  (`self.Fire Shot`)
  (`KismetSystemLibrary.Delay` (`self.Time between shots`))
  (if (`self.isFiring`)
    (`self.Fire (Server)`)))

(event `Set Shooting (Server)`
  (params (Shooting :type Boolean))
  ;[1 1 1] Firing Shots
  (bind _output_get (set `self.isFiring` Shooting))
  (if _output_get
    (`self.Fire (Server)`)))

(event `Reload`
  ;[1 1 1] Clientside
  (`self.Reload (ServeR)`))

(event `Impact (Multicast)`
  (params (`Impact Locations` :type "Array of Vector Structure"))
  ;[1 1 1] Multicast FX
  (if (not (`KismetSystemLibrary.IsDedicatedServer`))
    (`self.FX Impact` `Impact Locations`)))

(event `Reload (ServeR)`
  ;[1 1 1] Reloading
  (`KismetSystemLibrary.Delay` (`self.ReloadSpeed`))
  (set `self.MagAmmo` (`self.MagazineSize`))
  (if (`self.isFiring`)
    (`self.Fire (Server)`)))

(event `Muzzleflash (Multicast)`
  ;[1 1 1] Multicast FX
  (if (not (`KismetSystemLibrary.IsDedicatedServer`))
    (`self.FX Muzzleflash` (`SceneComponent.K2_GetComponentLocation` (`self.Muzzle`)))))

(fn `Fire Shot`
  (bind _returnvalue (`SceneComponent.K2_GetComponentLocation` (`self.Muzzle`)))
  (`self.Muzzleflash (Multicast)`)
  (bind _outhit (`KismetSystemLibrary.LineTraceSingle` _returnvalue (+ _returnvalue (* (`KismetMathLibrary.RandomUnitVectorInConeInDegrees` (`self.GetActorForwardVector`) (`KismetMathLibrary.DegAtan` (/ (`self.Accuracy At 100m`) 100.0))) (`self.MaxRange`))) "TraceTypeQuery1" false (`|MakeArray` (`self.GetOwner`)) "ForDuration"))
  (`/Engine/EditorBlueprintResources/StandardMacros.DecrementInt` (`self.MagAmmo`)
    (:`  `
      (bind (_bblockinghit _binitialoverlap _time _distance _location _impactpoint _normal _impactnormal _physmat _hitactor) (`GameplayStatics.BreakHitResult` _outhit))
      (if _bblockinghit
        (`self.Impact (Multicast)` (`|MakeArray` _location))
        (`GameplayStatics.ApplyDamage` _hitactor (`KismetMathLibrary.Conv_IntToDouble` (`self.Damage`)))
        (return)
        (else
          (return))))))

(fn `FX Impact`
  (params (`Impact Locations` :type "Array of Vector Structure"))
  (`GameplayStatics.SpawnEmitterAtLocation` "/Game/StarterContent/Particles/P_Fire.P_Fire" (`|GetArrayItem` `Impact Locations`)))

(fn `FX Muzzleflash`
  (params (Location :type "Vector Structure"))
  (`GameplayStatics.SpawnEmitterAtLocation` "/Game/StarterContent/Particles/P_Explosion.P_Explosion" Location))

(fn `UserConstructionScript`)