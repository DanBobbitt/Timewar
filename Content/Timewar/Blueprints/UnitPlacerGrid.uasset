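; Unit placement designator that previews the cursor's held units as a formation of phantom waypoints, then spawns or cancels them.
; On BeginPlay it takes the player's units and spawns one waypoint each.
; Each tick it faces the cursor hit, widens rows with cursor distance, and positions waypoints via newly added arrow components.
; PlaceUnits spawns and registers units at waypoints not overlapping cover; CancelPlacement returns all units to the lobby palette.
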(event `self.ReceiveBeginPlay`
  (bind _units (`/Game/Timewar/Widgets/ScreenElements/Crosshair.RemoveAllUnits` (`/Game/Timewar/Blueprints/TW_PlayerController_Lobby.Cursor` (`self.ControllingPlayer`))))
  (bind _output_get (set `self.Units` _units))
  (for _array_element _output_get
    (bind (_unitclass _count) (break `/Game/Timewar/Structs/Unit` _array_element))
    (for _ (range 1 (+ _count 1))
      (bind _returnvalue (`|SpawnActorFromClass` "/Game/Timewar/Blueprints/PhantomPlacementWaypoint.PhantomPlacementWaypoint_C" (`self.GetTransform`) "AlwaysSpawn" "OverrideRootScale" null (make `/Game/Timewar/Structs/Unit` _unitclass) null))
      (`KismetArrayLibrary.Array_Add` (`self.PlacementWaypoints`) _returnvalue))))

(event `self.ReceiveTick`
  (params (DeltaSeconds :type "Float (single-precision)"))
  (`self.Update`))

(fn `CancelPlacement`
  (for _array_element (`self.Units`)
    (bind (_unitclass _count) (break `/Game/Timewar/Structs/Unit` _array_element))
    (for _ (range 1 (+ _count 1))
      (`/Game/Timewar/Widgets/ScreenElements/UnitPalette.AddUnitToPalette` (`/Game/Timewar/Widgets/Screens/LobbyMenu.UnitPalette` (`/Game/Timewar/Blueprints/TW_PlayerController_Lobby.LobbyWidget` (`self.ControllingPlayer`))) (make `/Game/Timewar/Structs/Unit` _unitclass))
      (for _array_element_2 (`self.PlacementWaypoints`)
        (`self.SetLifeSpan` _array_element_2 0.1)))))

(fn `GetClosestEntryPoint`
  (params (Cover :type "/Game/Timewar/Blueprints/Structures+Cover/Cover_Base Object Reference") (Unit :type "/Game/Timewar/Blueprints/Units/Unit_Base Object Reference"))
  (returns (NewParam :type "Vector Structure"))
  (locals (distance :type "Float (double-precision)" :default 100000000.0) (entrypoint :type "/Game/Timewar/Blueprints/Structures+Cover/EntryPoint Object Reference"))
  (for _array_element (`/Game/Timewar/Blueprints/Structures+Cover/Cover_Base.EntryPoints` Cover)
    (bind _returnvalue (`KismetMathLibrary.VSize` (- (`SceneComponent.K2_GetComponentLocation` _array_element) (`self.K2_GetActorLocation` Unit))))
    (if (< _returnvalue (`local.distance`))
      (set `local.distance` _returnvalue)
      (set `local.entrypoint` _array_element)))
  (return (`SceneComponent.K2_GetComponentLocation` (`local.entrypoint`))))

(fn `PlaceUnits`
  (for _array_element (`self.PlacementWaypoints`)
    (`/Engine/EditorBlueprintResources/StandardMacros.IsValid` (`/Game/Timewar/Blueprints/PhantomPlacementWaypoint.OverlappedCover` _array_element)
      (:`Is Not Valid`
        (bind _returnvalue (`|SpawnActorFromClass` (`.UnitClass_4_DE9684274FE455363CD46BA63A4C5974` (break `/Game/Timewar/Structs/Unit` (`/Game/Timewar/Blueprints/PhantomPlacementWaypoint.OwningUnit` _array_element))) (`self.GetTransform` _array_element) "AdjustIfPossibleButAlwaysSpawn" "OverrideRootScale" null null))
        (`/Game/Timewar/Blueprints/TW_GameState.Register Unit` (cast `/Game/Timewar/Blueprints/TW_GameState` (`GameplayStatics.GetGameState`) :!pure true) _returnvalue)
        (`self.SetLifeSpan` _array_element 0.01)))))

(fn `Update`
  (locals (Rows :type "Array of Integer") (RowIndex :type Integer))
  (bind _spread (`self.Spread`))
  (bind _spread_2 (`self.Spread`))
  (bind _returnvalue (`SceneComponent.K2_GetComponentLocation` (`self.DefaultSceneRoot`)))
  (bind _hitresult (`PlayerController.GetHitResultUnderCursorByChannel` (`self.ControllingPlayer`) "TraceTypeQuery1" false))
  (bind _returnvalue_2 (* 2 (`KismetMathLibrary.FTrunc` (/ (`KismetMathLibrary.VSize` (- (`.Location` (`GameplayStatics.BreakHitResult` _hitresult)) _returnvalue)) 1000.0))))
  ;[1 1 1] Set Designator rotation based on player's cursor.
  (if (== 0 _returnvalue_2)
    (`self.K2_SetActorRotation` (`KismetMathLibrary.FindLookAtRotation` _returnvalue _returnvalue))
    (else
      (`self.K2_SetActorRotation` (`KismetMathLibrary.FindLookAtRotation` _returnvalue (`.Location` (`GameplayStatics.BreakHitResult` _hitresult))))))
  ;[1 1 1] Increase number of columns the further the cursor is from the designator.
  (set `self.MaxColumnsInRow` (+ _returnvalue_2 1))
  (for _array_element (`self.PlacementWaypoints`)
    (if (== (`KismetArrayLibrary.Array_Length` (`local.Rows`)) 0)
      (`KismetArrayLibrary.Array_Add` (`local.Rows`))
      (bind _returnvalue_3 (`AddComponent|NODE_AddArrowComponent-0`))
      (`self.K2_SetActorTransform` _array_element (`SceneComponent.K2_GetComponentToWorld` _returnvalue_3) false false)
      (elif (== (`|GetArrayItem` (`local.Rows`) (`local.RowIndex`)) (`self.MaxColumnsInRow`))
        (`KismetArrayLibrary.Array_Add` (`local.Rows`))
        (bind _result (`/Engine/EditorBlueprintResources/StandardMacros.IncrementInt` (`local.RowIndex`))
          (:`  `
            (bind _returnvalue_4 (`AddComponent|NODE_AddArrowComponent-1` :`RelativeTransform` (`KismetMathLibrary.MakeTransform` (`KismetMathLibrary.MakeVector` (* (* _result -1) (`self.Spread`))))))
            (`self.K2_SetActorTransform` _array_element (`SceneComponent.K2_GetComponentToWorld` _returnvalue_4) false false)))
        (else
          (bind _result_2 (`/Engine/EditorBlueprintResources/StandardMacros.IncrementInt` (`|GetArrayItem` (`local.Rows`) (`local.RowIndex`)))
            (:`  `
              (if (== (mod _result_2 2) 0)
                (bind _returnvalue_5 (`AddComponent|NODE_AddArrowComponent-2` :`RelativeTransform` (`KismetMathLibrary.MakeTransform` (`KismetMathLibrary.MakeVector` (* (* (`local.RowIndex`) -1) _spread_2) (* (/ (`|GetArrayItem` (`local.Rows`) (`local.RowIndex`)) -2) _spread_2)))))
                (`self.K2_SetActorTransform` _array_element (`SceneComponent.K2_GetComponentToWorld` _returnvalue_5) false false)
                (else
                  (bind _returnvalue_6 (`AddComponent|NODE_AddArrowComponent-3` :`RelativeTransform` (`KismetMathLibrary.MakeTransform` (`KismetMathLibrary.MakeVector` (* (* (`local.RowIndex`) -1) _spread) (* (/ (+ (`|GetArrayItem` (`local.Rows`) (`local.RowIndex`)) 1) 2) _spread)))))
                  (`self.K2_SetActorTransform` _array_element (`SceneComponent.K2_GetComponentToWorld` _returnvalue_6) false false))))))))))

(fn `UserConstructionScript`)