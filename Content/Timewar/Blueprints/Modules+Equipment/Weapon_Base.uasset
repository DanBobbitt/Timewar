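; Base weapon for a unit's module that fires server-side bursts of hitscan shots at the parent module's current target.
; A randomly timed attack loop checks facing, then runs recursive salvos that reload when the magazine empties.
; On authority, Tick drifts an aimpoint around the target by unit accuracy and range.
; Shots trace within a precision cone toward it, sending kinetic damage and multicasting muzzle and impact FX.
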(event `Salvo (Server)`
  (bind _burstamount (`self.BurstAmount`))
  (bind _magazinesize (`self.MagazineSize`))
  ;[1 1 1] Firing Shots
  (if (and (== (`self.burstindex`) 0) (`KismetSystemLibrary.IsValid` (`/Game/Timewar/Blueprints/Modules+Equipment/Module_Base.CurrentTarget` (`self.Parent Module`))))
    (if (not (`self.EnforcedBurstAmount`))
      (set `self.burstcount` (`KismetMathLibrary.RandomIntegerInRange` (`KismetMathLibrary.Clamp` (+ _burstamount 3) 0 _magazinesize) (`KismetMathLibrary.Clamp` (- _burstamount 3) 0 _magazinesize))))
    (`self.Fire Shot` :!label _label)
    (bind _result (`/Engine/EditorBlueprintResources/StandardMacros.IncrementInt` (`self.burstindex`))
      (:`  `
        (if (< _result (`self.BurstAmount`))
          (if (> (`self.MagAmmo`) 0)
            (`KismetSystemLibrary.Delay` (`self.Firerate`))
            (`self.Salvo Recursive (Server)`)
            (else
              (set `self.burstindex` 0)
              (`self.Reload (Server)`)))
          (else
            (set `self.burstindex` 0)))))))

(event `Salvo Recursive (Server)`
  ;[1 1 1] Firing Shots
  (goto _label))

(event `Attempt Fire (Server)`
  (bind _attackspersecond (`/Game/Timewar/Blueprints/Units/Unit_Base.AttacksPerSecond` (`/Game/Timewar/Blueprints/Modules+Equipment/Module_Base.ParentUnit` (`self.Parent Module`))))
  ;[1 1 1] Firing Shots
  (`self.WeaponCanFire`
    (:`true`
      (`self.Salvo (Server)`))
    (:`false`
      _))
  (`KismetSystemLibrary.Delay` (`KismetMathLibrary.RandomFloatInRange` (* _attackspersecond 0.5) (* _attackspersecond 1.5)))
  (if (`self.isFiring`)
    (`self.Attempt Fire (Server)`)))

(event `Set Shooting`
  (params (Shooting :type Boolean))
  ;[1 1 1] Clientside (Direct Control Only)
  (`self.Toggle Firing (Server)` Shooting))

(event `Toggle Firing (Server)`
  (params (Shooting :type Boolean))
  ;[1 1 1] Firing Shots
  (bind _output_get (set `self.isFiring` Shooting))
  (if _output_get
    (`/Engine/EditorBlueprintResources/StandardMacros.DoOnce` false :!label _label_2
      (:`Completed`
        (`self.Attempt Fire (Server)`)))
    (else
      (goto _label_2 :!via `Reset`))))

(event `Reload`
  ;[1 1 1] Clientside (Direct Control Only)
  (`self.Reload (ServeR)`))

(event `Impact (Multicast)`
  (params (`Impact Locations` :type "Vector Structure"))
  ;[1 1 1] Multicast FX
  (if (not (`KismetSystemLibrary.IsDedicatedServer`))
    (`self.FX Impact` `Impact Locations`)))

(event `self.ReceiveTick`
  (params (DeltaSeconds :type "Float (single-precision)"))
  (`/Engine/EditorBlueprintResources/ActorMacros.Switch Has Authority`
    (:`Authority`
      (`self.UpdateWeaponDeviation` DeltaSeconds))))

(event `Reload (Server)`
  ;[1 1 1] Reloading
  (`KismetSystemLibrary.Delay` (`self.ReloadSpeed`))
  (set `self.MagAmmo` (`self.MagazineSize`))
  (if (`self.isFiring`)
    (`self.Attempt Fire (Server)`)))

(event `Muzzleflash (Multicast)`
  ;[1 1 1] Multicast FX
  (if (not (`KismetSystemLibrary.IsDedicatedServer`))
    (`self.FX Muzzleflash` (`SceneComponent.K2_GetComponentLocation` (`self.Muzzle`)))))

(fn `Fire Shot`
  (bind _returnvalue (`SceneComponent.K2_GetComponentLocation` (`self.Muzzle`)))
  (`self.Muzzleflash (Multicast)`)
  (bind _outhit (`KismetSystemLibrary.LineTraceSingle` _returnvalue (+ _returnvalue (* (`KismetMathLibrary.RandomUnitVectorInConeInDegrees` (`KismetMathLibrary.GetDirectionUnitVector` (`SceneComponent.K2_GetComponentLocation` (`self.Muzzle`)) (`SceneComponent.K2_GetComponentLocation` (`self.Aimpoint`))) (`KismetMathLibrary.DegAtan` (/ (`self.PrecisionInMetersAt100m`) 100.0))) (* (`self.MaxRange`) 1.5))) "TraceTypeQuery3" false (`/Game/Timewar/Blueprints/Units/Unit_Base.ModuleActors` (`/Game/Timewar/Blueprints/Modules+Equipment/Module_Base.ParentUnit` (`self.Parent Module`))) "None" true (struct :`R` 1.0 :`A` 1.0) (struct :`G` 1.0 :`A` 1.0) 0.1))
  (`/Engine/EditorBlueprintResources/StandardMacros.DecrementInt` (`self.MagAmmo`)
    (:`  `
      (bind (_bblockinghit _binitialoverlap _time _distance _location _impactpoint _normal _impactnormal _physmat _hitactor) (`GameplayStatics.BreakHitResult` _outhit))
      (if _bblockinghit
        (`self.Impact (Multicast)` _location)
        (message `/Game/Timewar/Blueprints/Core/Damageable.Recieve Attack` _hitactor (`self.Damage`) (`self.Penetration`) "Kinetic")
        (return)
        (else
          (return))))))

(fn `FX Impact`
  (params (`Impact Locations` :type "Vector Structure"))
  (`GameplayStatics.SpawnEmitterAtLocation` "/Game/StarterContent/Particles/P_Explosion.P_Explosion" `Impact Locations`))

(fn `FX Muzzleflash`
  (params (Location :type "Vector Structure")))

(fn `UserConstructionScript`
  (set `self.MagAmmo` (`self.MagazineSize`))
  (`SceneComponent.SetAbsolute` (`self.TargetPoint`) true true true))