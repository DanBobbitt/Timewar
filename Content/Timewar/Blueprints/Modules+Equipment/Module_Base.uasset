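; Base module actor for a Unit_Base, acting as one formation member that carries equipment and engages the unit's target.
; On BeginPlay it spawns socketed equipment, records the longest weapon range and sorts by point value.
; While the unit moves, it drifts toward randomised offsets around its formation slot, snapping to ground via line trace.
; It turns toward in-range targets, otherwise matches the unit token, with weapon firing toggled on authority.
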(event `self.ReceiveTick`
  (params (DeltaSeconds :type "Float (single-precision)"))
  (`/Engine/EditorBlueprintResources/StandardMacros.IsValid` (`self.ParentUnit`)
    (:`Is Valid`
      (`self.UpdatePosition` DeltaSeconds)
      (`self.AimAndEngageTarget` DeltaSeconds))))

(event `Update Desired Offset`
  (params (`Random X` :type "Float (double-precision)") (`Random Y` :type "Float (double-precision)") (Radius :type "Float (double-precision)"))
  (set `self.(Relative) Desired Offset` (+ (`self.(Relative) Formation Slot`) (* (`KismetMathLibrary.MakeVector` `Random X` `Random Y`) Radius))))

(event `self.ReceiveBeginPlay`
  (bind _asunit_base (cast `/Game/Timewar/Blueprints/Units/Unit_Base` (`self.GetParentActor`)))
  (set `self.ParentUnit` _asunit_base)
  (`self.SpawnAndAttachEquipment`)
  (`self.Update Desired Offset` (`KismetMathLibrary.RandomFloatInRange` -1.0 1.0) (`KismetMathLibrary.RandomFloatInRange` -1.0 1.0) 100.0))

(fn `SpawnAndAttachEquipment`
  (for _array_element (`self.EquipmentSlots`)
    (bind _aspawn (cast `Pawn` (`self.GetParentActor`))
      (:`then`
        (bind _returnvalue (`|SpawnActorFromClass` (break `/Game/Timewar/Blueprints/Modules+Equipment/EquipmentSlot` _array_element) (`self.GetTransform`) "AlwaysSpawn" "OverrideRootScale" null _aspawn))
        (`self.K2_AttachToComponent` _returnvalue (`self.Mesh`) (`.SocketName_27_AA068AC44829C3BD18A28D8C52975812` (break `/Game/Timewar/Blueprints/Modules+Equipment/EquipmentSlot` _array_element)) "SnapToTarget" "SnapToTarget" "SnapToTarget" true)
        (`KismetArrayLibrary.Array_Add` (`self.Equipment`) _returnvalue)
        (set `/Game/Timewar/Blueprints/Modules+Equipment/Equipment_Base.Parent Module` self _returnvalue)
        (bind _asweapon_base (cast `/Game/Timewar/Blueprints/Modules+Equipment/Weapon_Base` _returnvalue))
        (bind _maxrange (`/Game/Timewar/Blueprints/Modules+Equipment/Weapon_Base.MaxRange` _asweapon_base))
        (if (> _maxrange (`self.LargestRange`))
          (set `self.LargestRange` _maxrange)))
      (:`CastFailed`
        (`KismetSystemLibrary.PrintString` "Module Not child of a Pawn actor! Failed to spawn equipment." true true (struct :`R` 1.0 :`G` 0.025124 :`A` 1.0) 10.0))))
  (`VictoryBPFunctionLibrary.Array_Sort` (`self.Equipment`) true "PointValue"))

(fn `UserConstructionScript`)