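; PhantomOrderWaypoint is an order waypoint actor that detects the cover it is placed over.
; Every tick it queries overlapping Cover_Base actors and stores a single match in OverlappedCover, clearing it when none overlap.
; Its sphere doubles in scale while over one cover as visual feedback.
; Overlapping several covers only prints a warning, leaving the previous state unchanged.
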(event `self.ReceiveTick`
  (params (DeltaSeconds :type "Float (single-precision)"))
  (bind _overlappingactors (`self.GetOverlappingActors` "/Game/Timewar/Blueprints/Structures+Cover/Cover_Base.Cover_Base_C"))
  (bind _returnvalue (`KismetArrayLibrary.Array_Length` _overlappingactors))
  (if (> _returnvalue 1)
    (`KismetSystemLibrary.PrintString` "Warning! Waypoint overlapping multiple Cover_Base! ")
    (elif (== _returnvalue 1)
      (`SceneComponent.SetWorldScale3D` (`self.Sphere`) (2.0 2.0 2.0))
      (set `self.OverlappedCover` (cast `/Game/Timewar/Blueprints/Structures+Cover/Cover_Base` (`|GetArrayItem` _overlappingactors) :!pure true))
      (else
        (`SceneComponent.SetWorldScale3D` (`self.Sphere`) (1.0 1.0 1.0))
        (set `self.OverlappedCover` null)))))

(fn `UserConstructionScript`)