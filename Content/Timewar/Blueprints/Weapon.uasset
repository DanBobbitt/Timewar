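; Unit weapon that automatically aims and fires at other Units within its range.
; A range sphere tracks potential targets without a team check; when the current target is invalid or memberless, FireAtWill seeks the closest.
; Tick uses delays to gate aiming and chambering while armed.
; Shots roll against Accuracy, either calling RecieveHit on the target or spawning an explosion at a randomly offset trace end.
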(event `self.ReceiveBeginPlay`
  (`SphereComponent.SetSphereRadius` (`self.MaxRangeSphere`) (`self.MaxRange`) true))

(event `self.ReceiveTick`
  (params (DeltaSeconds :type "Float (single-precision)"))
  (`self.CurrentTargetValid?`
    (:`Valid`
      (if (and (`self.Aimed?`) (`self.Armed?`))
        (if (`self.Chambered?`)
          (`self.FireShot`)
          (set `self.Chambered?` false)
          (else
            (`KismetSystemLibrary.Delay` (`self.Time between shots`))
            (set `self.Chambered?` true)))
        (else
          (`KismetSystemLibrary.Delay` (`self.Time to aim`))
          (set `self.Aimed?` true))))
    (:`Invalid`
      (`KismetArrayLibrary.Array_RemoveItem` (`self.PotentialTargets`) (`self.CurrentTarget`))
      (if (`self.FireAtWill`)
        (`self.EngageClosestTarget`)))))

(event `self.MaxRangeSphere.OnComponentBeginOverlap`
  (params (OverlappedComponent :type "PrimitiveComponent Object Reference") (OtherActor :type "Actor Object Reference") (OtherComp :type "PrimitiveComponent Object Reference") (OtherBodyIndex :type Integer) (bFromSweep :type Boolean) (SweepResult :type "HitResult Structure (by ref)"))
  (bind _asunit (cast `/Game/Timewar/Blueprints/Units/Unit` OtherActor))
  (if (not (== (`self.Owning Unit`) _asunit))
    (`KismetArrayLibrary.Array_Add` (`self.PotentialTargets`) _asunit)))

(event `self.MaxRangeSphere.OnComponentEndOverlap`
  (params (OverlappedComponent :type "PrimitiveComponent Object Reference") (OtherActor :type "Actor Object Reference") (OtherComp :type "PrimitiveComponent Object Reference") (OtherBodyIndex :type Integer))
  (bind _asunit (cast `/Game/Timewar/Blueprints/Units/Unit` OtherActor))
  (`KismetArrayLibrary.Array_RemoveItem` (`self.PotentialTargets`) _asunit)
  (if (== (`self.CurrentTarget`) _asunit)
    (set `self.CurrentTarget` null)
    (set `self.Aimed?` false)))

(event `Safe Weapon`
  (set `self.Armed?` false))

(event `Arm Weapon`
  (set `self.Armed?` true))

(fn `EngageClosestTarget`
  (locals (distance :type "Float (double-precision)" :default 100000000.0))
  (for _array_element (`self.PotentialTargets`)
    (bind _returnvalue (`self.GetDistanceTo` _array_element self))
    (if (< _returnvalue (`local.distance`))
      (set `local.distance` _returnvalue)
      (set `self.CurrentTarget` _array_element))))

(fn `FireShot`
  (locals (hit :type "Float (double-precision)"))
  (`/Engine/EditorBlueprintResources/StandardMacros.IsValid` (`self.CurrentTarget`)
    (:`Is Valid`
      (bind _output_get (set `local.hit` (`KismetMathLibrary.RandomFloatInRange` 0.0 1.0)))
      (if (> (`self.Accuracy`) _output_get)
        (`/Game/Timewar/Blueprints/Units/Unit.RecieveHit` (`self.CurrentTarget`) self)
        (else
          (`self.GenerateMiss` self))))))

(fn `GenerateMiss`
  (bind _unitradius (`/Game/Timewar/Blueprints/Units/Unit.UnitRadius` (`self.CurrentTarget`)))
  (bind _unitradius_2 (`/Game/Timewar/Blueprints/Units/Unit.UnitRadius` (`self.CurrentTarget`)))
  (bind _outhit (`KismetSystemLibrary.LineTraceSingle` :`Start` (`SceneComponent.K2_GetComponentLocation` (`self.Cube`)) :`End` (+ (`SceneComponent.K2_GetComponentLocation` (`/Game/Timewar/Blueprints/Units/Unit.UnitRadius` (`self.CurrentTarget`))) (`KismetMathLibrary.MakeVector` (`KismetMathLibrary.RandomFloatInRange` (* (`SphereComponent.SphereRadius` _unitradius_2) -1.0) (`SphereComponent.SphereRadius` _unitradius_2)) (`KismetMathLibrary.RandomFloatInRange` (* (`SphereComponent.SphereRadius` _unitradius) -2.0) (* (`SphereComponent.SphereRadius` _unitradius) 2.0)) -100.0)) :`TraceChannel` "TraceTypeQuery3" :`DrawTime` 0.2))
  (`GameplayStatics.SpawnEmitterAtLocation` "/Game/StarterContent/Particles/P_Explosion.P_Explosion" (`.TraceEnd` (`GameplayStatics.BreakHitResult` _outhit))))

(fn `UserConstructionScript`)