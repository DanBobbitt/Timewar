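; HUD for mouse box-selection of units, with an on-screen name label over every Unit.
; Each DrawHUD frame draws a rectangle from drag start to cursor while left mouse is held, using paired DoOnce latches to capture press and release.
; On release it passes both corners to the Player controller's BoxSelect.
; It also fetches all Units every frame and draws their object names at projected positions, gold if selected, otherwise team-coloured.
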(event `self.ReceiveBeginPlay`
  (bind _asplayer (cast `/Game/Timewar/Blueprints/Core/Players/Player` (`self.GetOwningPlayerController`)))
  (set `self.MyPlayerController` _asplayer))

(event `self.ReceiveDrawHUD`
  (params (SizeX :type Integer) (SizeY :type Integer))
  (`/Engine/EditorBlueprintResources/StandardMacros.IsValid` (`self.MyPlayerController`)
    (:`Is Valid`
      (`|ExecutionSequence`
        (:`then_0`
          (`self.Selection Box`))
        (:`then_1`
          (`self.Render Unit Icons`))))))

(fn `UserConstructionScript`)