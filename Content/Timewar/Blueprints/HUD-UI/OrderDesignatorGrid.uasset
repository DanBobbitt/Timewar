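; RTS formation-order preview actor that lays out one marker per selected unit in a grid anchored at its location.
; Initialize spawns the markers as child actor components.
; Each tick, the grid turns toward the cursor hit, widens rows with cursor distance, and fills them alternately either side of centre, stacking further rows behind.
; ExecuteOrder sends each selected unit to its index-matched marker, with Shift queuing and A attack-moving.
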(event `self.ReceiveTick`
  (params (DeltaSeconds :type "Float (single-precision)"))
  (`self.Update`))

(fn `ExecuteOrder`
  (bind _controllingplayer (`self.ControllingPlayer`))
  (for (_array_element _array_index) (`/Game/Timewar/Blueprints/Core/Players/Player.CurrentlySelectedUnits` _controllingplayer)
    (`/Game/Timewar/Blueprints/Core/Players/Player.Send Unit an Order` (`self.ControllingPlayer`) _array_element (`PlayerController.IsInputKeyDown` _controllingplayer "LeftShift") (`PlayerController.IsInputKeyDown` _controllingplayer "A") (`SceneComponent.K2_GetComponentLocation` (`|GetArrayItem` (`self.Unit Order Markers`) _array_index)) null)))

(fn `Initialize`
  (params (PlayerController :type "/Game/Timewar/Blueprints/Core/Players/Player Object Reference") (SelectedUnits :type "Array of /Game/Timewar/Blueprints/Units/Unit Object Reference"))
  (set `self.ControllingPlayer` PlayerController)
  (for _ SelectedUnits
    (bind _returnvalue (`AddComponent|NODE_AddChildActorComponent-0` :`RelativeTransform` (`SceneComponent.K2_GetComponentToWorld` (`self.DefaultSceneRoot`))))
    (`ChildActorComponent.SetChildActorClass` _returnvalue "/Game/Timewar/Blueprints/HUD-UI/UnitOrderMarker.UnitOrderMarker_C")
    (`KismetArrayLibrary.Array_Add` (`self.Unit Order Markers`) _returnvalue)))

(fn `Update`
  (locals (Rows :type "Array of Integer") (RowIndex :type Integer))
  (bind _spread (`self.Spread`))
  (bind _spread_2 (`self.Spread`))
  (bind _returnvalue (`SceneComponent.K2_GetComponentLocation` (`self.DefaultSceneRoot`)))
  (bind _hitresult (`PlayerController.GetHitResultUnderCursorByChannel` (`self.ControllingPlayer`) "TraceTypeQuery1" false))
  (set `self.MaxColumnsInRow` (+ 2 (* (`KismetMathLibrary.FTrunc` (/ (`KismetMathLibrary.VSize` (- (`.Location` (`GameplayStatics.BreakHitResult` _hitresult)) _returnvalue)) 1000.0)) 2)))
  (`self.K2_SetActorRotation` (`KismetMathLibrary.FindLookAtRotation` _returnvalue (`.Location` (`GameplayStatics.BreakHitResult` _hitresult))))
  (for _array_element (`self.Unit Order Markers`)
    (if (== (`KismetArrayLibrary.Array_Length` (`local.Rows`)) 0)
      (`KismetArrayLibrary.Array_Add` (`local.Rows`))
      (`SceneComponent.K2_SetRelativeTransform` _array_element (`KismetMathLibrary.MakeTransform` (0.0 0.0 0.0)) false true)
      (elif (== (`|GetArrayItem` (`local.Rows`) (`local.RowIndex`)) (`self.MaxColumnsInRow`))
        (`KismetArrayLibrary.Array_Add` (`local.Rows`))
        (bind _result (`/Engine/EditorBlueprintResources/StandardMacros.IncrementInt` (`local.RowIndex`))
          (:`  `
            (`SceneComponent.K2_SetRelativeTransform` _array_element (`KismetMathLibrary.MakeTransform` (`KismetMathLibrary.MakeVector` (* (* _result -1) (`self.Spread`)))) false true)))
        (else
          (bind _result_2 (`/Engine/EditorBlueprintResources/StandardMacros.IncrementInt` (`|GetArrayItem` (`local.Rows`) (`local.RowIndex`)))
            (:`  `
              (if (== (mod _result_2 2) 0)
                (`SceneComponent.K2_SetRelativeTransform` _array_element (`KismetMathLibrary.MakeTransform` (`KismetMathLibrary.MakeVector` (* (* (`local.RowIndex`) -1) _spread_2) (* (/ (`|GetArrayItem` (`local.Rows`) (`local.RowIndex`)) -2) _spread_2))) false true)
                (else
                  (`SceneComponent.K2_SetRelativeTransform` _array_element (`KismetMathLibrary.MakeTransform` (`KismetMathLibrary.MakeVector` (* (* (`local.RowIndex`) -1) _spread) (* (/ (+ (`|GetArrayItem` (`local.Rows`) (`local.RowIndex`)) 1) 2) _spread))) false true))))))))))

(fn `UserConstructionScript`)