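; PhantomPlacementWaypoint is a placement marker for a unit's waypoint that detects the cover it sits on.
; On BeginPlay it builds a UnitWidget for its owning unit, shows it on the widget component and switches it to a fixed panel.
; Each tick it polls overlapping Cover_Base actors, enlarging its sphere and storing the cover for a single overlap, resetting both for none, and printing a warning for several.
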(event `self.ReceiveBeginPlay`
  (bind _widget (`self.Widget`))
  (bind _returnvalue (`|CreateWidget` "/Game/Timewar/Widgets/ModularObjects/UnitWidget.UnitWidget_C" null (`self.OwningUnit`) null))
  (`WidgetComponent.SetWidget` _widget _returnvalue)
  (`WidgetSwitcher.SetActiveWidgetIndex` (`/Game/Timewar/Widgets/ModularObjects/UnitWidget.WidgetSwitcher_0` (cast `/Game/Timewar/Widgets/ModularObjects/UnitWidget` (`WidgetComponent.GetUserWidgetObject` _widget) :!pure true)) 6))

(event `self.ReceiveTick`
  (params (DeltaSeconds :type "Float (single-precision)"))
  (bind _overlappingactors (`self.GetOverlappingActors` "/Game/Timewar/Blueprints/Structures+Cover/Cover_Base.Cover_Base_C"))
  (bind _returnvalue (`KismetArrayLibrary.Array_Length` _overlappingactors))
  (if (> _returnvalue 1)
    (`KismetSystemLibrary.PrintString` "Warning! Waypoint overlapping multiple Cover_Base! ")
    (elif (== _returnvalue 1)
      (`SceneComponent.SetWorldScale3D` (`self.Sphere`) (2.0 2.0 2.0))
      (set `self.OverlappedCover` (cast `/Game/Timewar/Blueprints/Structures+Cover/Cover_Base` (`|GetArrayItem` _overlappingactors) :!pure true))
      (else
        (`SceneComponent.SetWorldScale3D` (`self.Sphere`) (1.0 1.0 1.0))
        (set `self.OverlappedCover` null)))))

(fn `UserConstructionScript`)