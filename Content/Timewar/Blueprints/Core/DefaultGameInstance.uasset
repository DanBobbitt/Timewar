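; Game instance for Timewar that drives menu flow and online session hosting, joining and teardown.
; A state machine in TransitionState removes the current screen's widget, or destroys the session when leaving Playing, before each show event displays its lazily created, cached widget.
; Hosting opens Level1 as a listen server, optionally over LAN.
; Session failures, travel errors and client-side network errors route to an error dialog that also destroys the session.
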(event `Show Loading Screen`
  ;[1 1 1] Show Loading Screen
  (`self.TransitionState` "NewEnumerator3"
    (:`Out`
      (bind _returnvalue (`self.Create or Get Loading Screen Widget`)
        (:`Is Valid`
          (`UserWidget.AddToViewport` _returnvalue 0)
          (`WidgetBlueprintLibrary.SetInputMode_UIOnlyEx` (`GameplayStatics.GetPlayerController` 0) _returnvalue))))))

(event `Show Main Menu`
  (bind _returnvalue (`GameplayStatics.GetPlayerController` 0))
  ;[1 1 1] Show Main Menu
  (if (`|EnumEquality` (`self.CurrentState`) "NewEnumerator5")
    (`GameplayStatics.OpenLevel` "MainMenu"))
  (`self.TransitionState` "NewEnumerator1"
    (:`Out`
      (`/Engine/EditorBlueprintResources/StandardMacros.IsValid` (`self.MainMenuWidget`)
        (:`Is Valid`
          _)
        (:`Is Not Valid`
          (bind _returnvalue_2 (`|CreateWidget` "/Game/Timewar/Blueprints/HUD-UI/Widgets/MainMenu.MainMenu_C" _returnvalue))
          (bind _output_get (set `self.MainMenuWidget` _returnvalue_2))))
      (`WidgetBlueprintLibrary.SetInputMode_UIOnlyEx` _returnvalue _output_get)
      (`UserWidget.AddToViewport` (`self.MainMenuWidget`) 0)
      (set `PlayerController.bShowMouseCursor` true _returnvalue))))

(event `Show Server list`
  ;[1 1 1] Show Server List
  (`self.TransitionState` "NewEnumerator2"
    (:`Out`
      (bind _server_list_widget (`self.Create or Get Server List Widget`))
      (`UserWidget.AddToViewport` _server_list_widget 0)
      (`WidgetBlueprintLibrary.SetInputMode_UIOnlyEx` (`GameplayStatics.GetPlayerController` 0) _server_list_widget))))

(event `Join From Server List`
  (params (SessionResult :type "BlueprintSessionResult Structure"))
  ;[1 1 1] Join From Server List
  (`self.Show Loading Screen`)
  (`JoinSessionCallbackProxy.JoinSession` (`GameplayStatics.GetPlayerController` 0) SessionResult
    (:`OnSuccess`
      (set `self.CurrentState` "NewEnumerator5"))
    (:`OnFailure`
      (`self.DisplayErrorDialogue` "Failed to join session."))))

(event `self.HandleNetworkError`
  (params (FailureType :type "ENetworkFailure Enum" :default "NetDriverAlreadyExists") (bIsServer :type Boolean))
  ;[1 1 1] Network errors (Called from code)
  (if (not bIsServer)
    (`self.DisplayErrorDialogue` (`|GetEnumeratorNameAsString` FailureType))))

(event `self.HandleTravelError`
  (params (FailureType :type "ETravelFailure Enum" :default "NoLevel"))
  ;[1 1 1] Network errors (Called from code)
  (`self.DisplayErrorDialogue` (`|GetEnumeratorNameAsString` FailureType)))

(event `Host Game`
  ;[1 1 1] Host Game
  (`self.Show Loading Screen`)
  (`CreateSessionCallbackProxy.CreateSession` (`GameplayStatics.GetPlayerController` 0) 2 (`self.EnableLan`)
    (:`OnSuccess`
      (set `self.CurrentState` "NewEnumerator5")
      (`GameplayStatics.OpenLevel` "Level1" true "listen"))
    (:`OnFailure`
      (`self.DisplayErrorDialogue` "Failed to create session."))))

(event `Destroy My Session`
  ;[1 1 1] Destroy My Session
  (`DestroySessionCallbackProxy.DestroySession` (`GameplayStatics.GetPlayerController` 0)))

(fn `Initialization`
  (if (`|EnumEquality` (`self.CurrentState`) "NewEnumerator0")
    (`self.Show Main Menu`)
    (else
      (`KismetSystemLibrary.PrintString` "Tried starting up but wasn't in Startup State!"))))