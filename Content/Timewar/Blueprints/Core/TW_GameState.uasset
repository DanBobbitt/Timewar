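; Game state for Timewar that keeps a registry of active units and decides which units each one can see.
; On the authority, a delay in Tick throttles visibility updates to roughly every quarter second.
; Each pass checks all unit pairs by vision radius and line trace, adding or removing relevant targets on each unit.
; Unregistering also clears the unit from others' targets; the pregame event only prints a delayed debug message.
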(event `self.ReceiveBeginPlay`)

(event `self.ReceiveTick`
  (params (DeltaSeconds :type "Float (single-precision)"))
  (`/Engine/EditorBlueprintResources/ActorMacros.Switch Has Authority`
    (:`Authority`
      (`KismetSystemLibrary.Delay` 0.25)
      (`self.UpdateUnitVisibility`))))

(event `Register Unit`
  (params (Unit :type "/Game/Timewar/Blueprints/Units/Unit_Base Object Reference"))
  (`KismetArrayLibrary.Array_Add` (`self.ActiveUnits`) Unit))

(event `Unregister Unit`
  (params (Unit :type "/Game/Timewar/Blueprints/Units/Unit_Base Object Reference"))
  (for _array_element (`self.ActiveUnits`)
    (`/Game/Timewar/Blueprints/Units/Unit_Base.RemoveRelevantTarget` _array_element Unit)
    (`KismetArrayLibrary.Array_RemoveItem` (`self.ActiveUnits`) Unit)))

(event `Begin Pregame`
  (`KismetSystemLibrary.Delay` 5.0)
  (`KismetSystemLibrary.PrintString` "5 seconds after pregame"))

(fn `UpdateUnitVisibility`
  (for _array_element (`self.ActiveUnits`)
    (for _array_element_2 (`self.ActiveUnits`)
      (if (< (`self.GetDistanceTo` _array_element_2 _array_element) (`/Game/Timewar/Blueprints/Units/Unit_Base.VisionRadius` _array_element))
        (bind (_outhit _returnvalue) (`KismetSystemLibrary.LineTraceSingle` :`Start` (`self.K2_GetActorLocation` _array_element) :`End` (`self.K2_GetActorLocation` _array_element_2) :`TraceChannel` "TraceTypeQuery5" :`DrawTime` 0.25))
        (if _returnvalue
          (`/Game/Timewar/Blueprints/Units/Unit_Base.RemoveRelevantTarget` _array_element _array_element_2 :!label _label)
          (else
            (`/Game/Timewar/Blueprints/Units/Unit_Base.AddRelevantTarget` _array_element _array_element_2)))
        (else
          (goto _label))))))

(fn `UserConstructionScript`)