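; Timewar game instance that owns the menu UI, online session flow and saved player info.
; A save check at startup loads player info and opens the main menu, or shows options if none exists.
; Menu widgets are created lazily and cached, while TransitionState removes the outgoing screen for loading and error changes.
; Hosting opens Lobby as a listen server; session, network and travel failures route to an error dialog that destroys the session.
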(event `SaveGameCheck`
  ;[1 1 1] Check Save game
  (bind _returnvalue (`GameplayStatics.DoesSaveGameExist` (`self.PlayerSettingsSave`)))
  (if _returnvalue
    (`self.LoadPlayerInfo`)
    (`self.Show Main Menu`)
    (set `self.SaveFileCreated?` true)
    (else
      (`self.ShowOptionsMenu`)
      (set `PlayerController.bShowMouseCursor` true (`GameplayStatics.GetPlayerController` 0)))))

(event `Show Loading Screen`
  ;[1 1 1] Show Loading Screen
  (`self.TransitionState` "NewEnumerator3"
    (:`Out`
      (bind _returnvalue (`self.Create or Get Loading Screen Widget`)
        (:`Is Valid`
          (`UserWidget.AddToViewport` _returnvalue 0)
          (`WidgetBlueprintLibrary.SetInputMode_UIOnlyEx` (`GameplayStatics.GetPlayerController` 0) _returnvalue))))))

(event `Show Main Menu`
  (bind _returnvalue (`GameplayStatics.GetPlayerController` 0))
  ;[1 1 1] Show Main Menu
  (`/Engine/EditorBlueprintResources/StandardMacros.IsValid` (`self.MainMenuWidget`)
    (:`Is Valid`
      _)
    (:`Is Not Valid`
      (bind _returnvalue_2 (`|CreateWidget` "/Game/Timewar/UI/Screens/MainMenu.MainMenu_C" _returnvalue))
      (bind _output_get (set `self.MainMenuWidget` _returnvalue_2))))
  (`WidgetBlueprintLibrary.SetInputMode_UIOnlyEx` _returnvalue _output_get)
  (`UserWidget.AddToViewport` (`self.MainMenuWidget`) 0)
  (set `PlayerController.bShowMouseCursor` true _returnvalue))

(event `Show Server list`
  ;[1 1 1] Show Server List
  (bind _server_list_widget (`self.Create or Get Server List Widget`))
  (`UserWidget.AddToViewport` _server_list_widget 0)
  (`WidgetBlueprintLibrary.SetInputMode_UIOnlyEx` (`GameplayStatics.GetPlayerController` 0) _server_list_widget))

(event `Join Session`
  (params (SessionResult :type "BlueprintSessionResult Structure"))
  ;[1 1 1] Join From Server List
  (`self.Show Loading Screen`)
  (`JoinSessionCallbackProxy.JoinSession` (`GameplayStatics.GetPlayerController` 0) SessionResult
    (:`OnSuccess`
      (set `self.CurrentState` "NewEnumerator5"))
    (:`OnFailure`
      (`self.DisplayErrorDialogue` "Failed to join session."))))

(event `self.HandleNetworkError`
  (params (FailureType :type "ENetworkFailure Enum" :default "NetDriverAlreadyExists") (bIsServer :type Boolean))
  ;[1 1 1] Network errors (Called from code)
  (if (not bIsServer)
    (`self.DisplayErrorDialogue` (`|GetEnumeratorNameAsString` FailureType))))

(event `self.HandleTravelError`
  (params (FailureType :type "ETravelFailure Enum" :default "NoLevel"))
  ;[1 1 1] Network errors (Called from code)
  (`self.DisplayErrorDialogue` (`|GetEnumeratorNameAsString` FailureType)))

(event `LaunchLobby`
  (params (NumberOfPlayers :type Integer) (ServerName :type Text) (EnableLAN :type Boolean))
  ;[1 1 1] Launch Lobby
  (set `self.MaxPlayers` NumberOfPlayers)
  (set `self.ServerName` ServerName)
  (`self.Show Loading Screen`)
  (`CreateSessionCallbackProxy.CreateSession` (`GameplayStatics.GetPlayerController` 0) (`self.MaxPlayers`) EnableLAN
    (:`OnSuccess`
      (set `self.CurrentState` "NewEnumerator5")
      (`GameplayStatics.OpenLevel` "Lobby" true "listen"))
    (:`OnFailure`
      (`self.DisplayErrorDialogue` "Failed to create lobby."))))

(event `Destroy My Session`
  (params (PlayerController :type "PlayerController Object Reference"))
  ;[1 1 1] Destroy My Session
  (`DestroySessionCallbackProxy.DestroySession` PlayerController))

(event `ShowHostMenu`
  ;[1 1 1] Host Game Menu
  (`/Engine/EditorBlueprintResources/StandardMacros.IsValid` (`self.HostMenu`)
    (:`Is Valid`
      _)
    (:`Is Not Valid`
      (bind _returnvalue (`|CreateWidget` "/Game/Timewar/UI/Screens/HostMenu.HostMenu_C" (`GameplayStatics.GetPlayerController` 0)))
      (set `self.HostMenu` _returnvalue)))
  (`UserWidget.AddToViewport` (`self.HostMenu`) 0))

(event `ShowOptionsMenu`
  ;[1 1 1] Options Menu
  (`/Engine/EditorBlueprintResources/StandardMacros.IsValid` (`self.OptionsMenu`)
    (:`Is Valid`
      _)
    (:`Is Not Valid`
      (bind _returnvalue (`|CreateWidget` "/Game/Timewar/UI/Screens/OptionsMenu.OptionsMenu_C" (`GameplayStatics.GetPlayerController` 0)))
      (set `self.OptionsMenu` _returnvalue)))
  (`UserWidget.AddToViewport` (`self.OptionsMenu`) 0))

(event `ShowMatchmakerMenu`
  ;[1 1 1] Matchmaker Menu
  (`/Engine/EditorBlueprintResources/StandardMacros.IsValid` (`self.MatchmakerMenu`)
    (:`Is Valid`
      _)
    (:`Is Not Valid`
      (bind _returnvalue (`|CreateWidget` "/Game/Timewar/UI/Screens/MatchmakerMenu.MatchmakerMenu_C" (`GameplayStatics.GetPlayerController` 0)))
      (set `self.MatchmakerMenu` _returnvalue)))
  (`UserWidget.AddToViewport` (`self.MatchmakerMenu`) 0))

(event `ShowArmyCustomizer`
  ;[1 1 1] CustomizerMenu
  (`/Engine/EditorBlueprintResources/StandardMacros.IsValid` (`self.ArmyCustomizer`)
    (:`Is Valid`
      _)
    (:`Is Not Valid`
      (bind _returnvalue (`|CreateWidget` "/Game/Timewar/UI/Screens/ArmyCustomizerMenu.ArmyCustomizerMenu_C" (`GameplayStatics.GetPlayerController` 0)))
      (set `self.ArmyCustomizer` _returnvalue)))
  (`UserWidget.AddToViewport` (`self.ArmyCustomizer`) 0))

(fn `LoadPlayerInfo`
  (bind _returnvalue (`GameplayStatics.LoadGameFromSlot` (`self.PlayerSettingsSave`)))
  (bind _astw_save_game (cast `/Game/Timewar/Blueprints/Core/TW_SaveGame` _returnvalue))
  (set `self.PlayerInfo` (`/Game/Timewar/Blueprints/Core/TW_SaveGame.SavedPlayerInfo` _astw_save_game)))

(fn `SavePlayerInfo`
  (bind _twsavegame (`self.TWSaveGame`))
  (`/Engine/EditorBlueprintResources/StandardMacros.IsValid` (`self.TWSaveGame`)
    (:`Is Valid`
      _)
    (:`Is Not Valid`
      (bind _returnvalue (`GameplayStatics.CreateSaveGameObject` "/Game/Timewar/Blueprints/Core/TW_SaveGame.TW_SaveGame_C"))
      (bind _astw_save_game (cast `/Game/Timewar/Blueprints/Core/TW_SaveGame` _returnvalue))
      (set `self.TWSaveGame` _astw_save_game)))
  (set `/Game/Timewar/Blueprints/Core/TW_SaveGame.SavedPlayerInfo` (`self.PlayerInfo`) _twsavegame)
  (`GameplayStatics.SaveGameToSlot` _twsavegame (`self.PlayerSettingsSave`)))