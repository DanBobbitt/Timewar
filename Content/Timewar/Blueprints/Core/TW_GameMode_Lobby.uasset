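; Lobby game mode that tracks joining players and match settings before a game starts.
; On login it registers each lobby controller, initializes it and sends it the current map image, name and time.
; UpdateAllPlayerInfo rebuilds the player info list, pushes counts and list to every controller, and sets CanWeStart from whether players have a named army selected.
; Host setting changes and game start are relayed by looping over all controllers.
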(event `self.K2_PostLogin`
  (params (NewPlayer :type "PlayerController Object Reference"))
  (bind _astw_player_controller_lobby (cast `/Game/Timewar/Blueprints/Core/TW_PlayerController_Lobby` NewPlayer :!pure true))
  ;[1 1 1] When a client logs in
  (`/Engine/EditorBlueprintResources/ActorMacros.Switch Has Authority`
    (:`Authority`
      (`KismetArrayLibrary.Array_Add` (`self.AllPlayerControllers`) _astw_player_controller_lobby)
      (`/Game/Timewar/Blueprints/Core/TW_PlayerController_Lobby.Post Login Server` _astw_player_controller_lobby)
      (`/Game/Timewar/Blueprints/Core/TW_PlayerController_Lobby.Post Login Client` _astw_player_controller_lobby (`self.ServerName`))
      (`self.UpdateAllPlayerInfo`)
      (`/Game/Timewar/Blueprints/Core/TW_PlayerController_Lobby.UpdateMatchSettings` _astw_player_controller_lobby (`self.GamemodeMapImage`) (`self.GamemodeMapName`) (`self.GamemodeMapTime`)))))

(event `UpdateAllPlayerInfo`
  (bind _allplayercontrollers (`self.AllPlayerControllers`))
  ;[1 1 1] Updates All Player's Lobby Information
  (bind _output_get (set `self.NumPlayers` (`KismetArrayLibrary.Array_Length` (`self.AllPlayerControllers`))))
  (if (> _output_get 0)
    (`KismetArrayLibrary.Array_Clear` (`self.ConnectedPlayerInfos`))
    (for _array_element _allplayercontrollers
      (bind _astw_player_controller_lobby (cast `/Game/Timewar/Blueprints/Core/TW_PlayerController_Lobby` _array_element))
      (bind _playerinfo (`/Game/Timewar/Blueprints/Core/TW_PlayerController_Lobby.PlayerInfo` _astw_player_controller_lobby))
      (`KismetArrayLibrary.Array_Add` (`self.ConnectedPlayerInfos`) _playerinfo)
      (`/Game/Timewar/Blueprints/Core/TW_PlayerController_Lobby.UpdateNumberOfPlayers` _astw_player_controller_lobby (`self.NumPlayers`) (`self.MaxPlayers`))
      (`KismetSystemLibrary.PrintText` (`.PlayerName_2_DDACA0A845940DE314CFD8983B132845` (break `/Game/Timewar/Blueprints/Core/PlayerInfo` _playerinfo))))
    (for _array_element_2 _allplayercontrollers
      (bind _astw_player_controller_lobby_2 (cast `/Game/Timewar/Blueprints/Core/TW_PlayerController_Lobby` _array_element_2))
      (`/Game/Timewar/Blueprints/Core/TW_PlayerController_Lobby.UpdatePlayerList` _astw_player_controller_lobby_2 (`self.ConnectedPlayerInfos`)))
    (for _array_element_3 (`self.ConnectedPlayerInfos`) :!label _label
      (if (`KismetTextLibrary.TextIsEmpty` (`.ArmyName_4_F57878CB4372AE4D42EE2398FEC5274B` (break `/Game/Timewar/Blueprints/Core/Army` (`.PlayerSelectedArmy_27_25758A2341875545717ABBA0F80333A1` (break `/Game/Timewar/Blueprints/Core/PlayerInfo` _array_element_3)))))
        (set `self.CanWeStart?` false)
        (`self.break`)
        (else
          (set `self.CanWeStart?` true))))
    (else
      (`KismetSystemLibrary.PrintString` "EverybodyUpdate: Number of players = 0!"))))

(event `Break`
  ;[1 1 1] Updates All Player's Lobby Information
  (goto _label :!via `Break`))

(event `ServerUpdateGameSettings`
  (params (MapImage :type "Texture2D Object Reference") (MapName :type Text) (MapTime :type Text))
  ;[1 1 1] Server made changes, update our lobby info for clients
  (set `self.GamemodeMapImage` MapImage)
  (set `self.GamemodeMapName` MapName)
  (set `self.GamemodeMapTime` MapTime)
  (for _array_element (`self.AllPlayerControllers`)
    (bind _astw_player_controller_lobby (cast `/Game/Timewar/Blueprints/Core/TW_PlayerController_Lobby` _array_element))
    (`/Game/Timewar/Blueprints/Core/TW_PlayerController_Lobby.UpdateMatchSettings` _astw_player_controller_lobby (`self.GamemodeMapImage`) (`self.GamemodeMapName`) (`self.GamemodeMapTime`))))

(event `Game Start`
  (for _array_element (`self.AllPlayerControllers`)
    (bind _astw_player_controller_lobby (cast `/Game/Timewar/Blueprints/Core/TW_PlayerController_Lobby` _array_element))
    (`/Game/Timewar/Blueprints/Core/TW_PlayerController_Lobby.Game Start` _astw_player_controller_lobby)))

(fn `UserConstructionScript`)