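; Base RTS unit character, assembled from child-actor modules, that dies on the server once its module list is empty.
; Construction registers the modules and records formation slots for one module type.
; Each server tick it picks the nearest relevant unit and has its modules target random modules on it, drawing a debug label.
; Orders form a waypoint-actor queue driven by AI SimpleMoveToActor, advancing on capsule overlap and facing the last waypoint's rotation.
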(event `self.ReceiveBeginPlay`)

(event `self.ReceiveTick`
  (params (DeltaSeconds :type "Float (single-precision)"))
  (bind _returnvalue (`self.GetVelocity`))
  (`/Engine/EditorBlueprintResources/ActorMacros.Switch Has Authority`
    (:`Authority`
      (if (== (`KismetArrayLibrary.Array_Length` (`self.Modules`)) 0)
        (`/Engine/EditorBlueprintResources/StandardMacros.DoOnce` false
          (:`Completed`
            (`self.Unit Death`)))
        (else
          (`self.Target Management On Tick`)
          (if (> (`KismetMathLibrary.VSize` _returnvalue) 10.0)
            (`SceneComponent.K2_SetWorldRotation` (`self.UnitToken`) (`KismetMathLibrary.MakeRotFromX` _returnvalue) false false)))))))

(event `Queue New Order`
  (params (`Clear Previous Orders` :type Boolean) (`Order Waypoint` :type "/Game/Timewar/Blueprints/Core/OrderWaypoint Object Reference"))
  (`self.Queue Order` `Clear Previous Orders` `Order Waypoint`))

(event `self.CapsuleComponent.OnComponentBeginOverlap`
  (params (OverlappedComponent :type "PrimitiveComponent Object Reference") (OtherActor :type "Actor Object Reference") (OtherComp :type "PrimitiveComponent Object Reference") (OtherBodyIndex :type Integer) (bFromSweep :type Boolean) (SweepResult :type "HitResult Structure (by ref)"))
  (`/Engine/EditorBlueprintResources/ActorMacros.Switch Has Authority`
    (:`Authority`
      (bind _asorder_waypoint (cast `/Game/Timewar/Blueprints/Core/OrderWaypoint` OtherActor))
      (`self.PassOverWaypoint` _asorder_waypoint))))

(fn `AddRelevantTarget`
  (params (`Target Actor` :type "Actor Object Reference (by ref)"))
  (bind _asunit_base (cast `/Game/Timewar/Blueprints/Units/Unit_Base` `Target Actor`))
  (if (not (== _asunit_base self))
    (`KismetArrayLibrary.Array_Add` (`self.RelevantTargets`) _asunit_base)))

(fn `Initialization`)

(fn `PassOverWaypoint`
  (params (`Order Waypoint` :type "/Game/Timewar/Blueprints/Core/OrderWaypoint Object Reference"))
  (bind _output (`|GetArrayItem` (`self.Waypoints`)))
  (if (== `Order Waypoint` _output)
    (if (> (`KismetArrayLibrary.Array_Length` (`self.Waypoints`)) 1)
      (`self.K2_DestroyActor` (`|GetArrayItem` (`self.Waypoints`)))
      (`KismetArrayLibrary.Array_Remove` (`self.Waypoints`))
      (`NavigationSystem.SimpleMoveToActor` (`AIBlueprintHelperLibrary.GetAIController` self) (`|GetArrayItem` (`self.Waypoints`)))
      (else
        (`SceneComponent.K2_SetWorldRotation` (`self.Mesh`) (`self.K2_GetActorRotation` _output) false false)
        (`self.K2_DestroyActor` (`|GetArrayItem` (`self.Waypoints`)))
        (`KismetArrayLibrary.Array_Remove` (`self.Waypoints`))
        (`MovementComponent.StopMovementImmediately` (`self.CharacterMovement`))))))

(fn `Queue Order`
  (params (`Clear Previous Order` :type Boolean) (`Order Waypoint` :type "/Game/Timewar/Blueprints/Core/OrderWaypoint Object Reference"))
  (if `Clear Previous Order`
    (for _array_element (`self.Waypoints`)
      (`self.K2_DestroyActor` _array_element))
    (`KismetArrayLibrary.Array_Clear` (`self.Waypoints`))
    (`KismetArrayLibrary.Array_Add` (`self.Waypoints`) `Order Waypoint`)
    (`NavigationSystem.SimpleMoveToActor` (`AIBlueprintHelperLibrary.GetAIController` self) (`|GetArrayItem` (`self.Waypoints`)) :!label _label)
    (else
      (bind _returnvalue (`KismetArrayLibrary.Array_Add` (`self.Waypoints`) `Order Waypoint`))
      (if (== _returnvalue 0)
        (goto _label)))))

(fn `RemoveRelevantTarget`
  (params (`Target Actor` :type "Actor Object Reference (by ref)"))
  (bind _asunit_base (cast `/Game/Timewar/Blueprints/Units/Unit_Base` `Target Actor`))
  (`KismetArrayLibrary.Array_RemoveItem` (`self.RelevantTargets`) _asunit_base)
  ;[1 1 1] Unset current target for relevant child modules
  (for _array_element (`self.Modules`)
    (if (== (`/Game/Timewar/Blueprints/Modules+Equipment/Module_Base.CurrentTarget` _array_element) _asunit_base)
      (set `/Game/Timewar/Blueprints/Modules+Equipment/Module_Base.CurrentTarget` null _array_element))))

(fn `Target Management On Tick`
  (locals (ClosestTargetRange :type "Float (double-precision)" :default 1000000000.0))
  (`KismetSystemLibrary.DrawDebugString` (`self.K2_GetActorLocation`) (`KismetSystemLibrary.GetDisplayName` (`self.CurrentTarget`)))
  (set `local.ClosestTargetRange` 100000000.0)
  (for _array_element (`self.RelevantTargets`)
    (bind _returnvalue (`self.GetDistanceTo` self _array_element))
    (if (< _returnvalue (`local.ClosestTargetRange`))
      (set `local.ClosestTargetRange` _returnvalue)
      (set `self.CurrentTarget` _array_element)
      (for _array_element_2 (`self.Modules`)
        (`/Game/Timewar/Blueprints/Modules+Equipment/Module_Base.Target Random Module` _array_element_2 _array_element)))))

(fn `ToggleSelected`
  (params (Selected :type Boolean))
  (bind _output_get (set `self.Selected?` Selected))
  (if _output_get
    _))

(fn `UserConstructionScript`
  ;[1 1 1] Spawn in our modules
  (for _array_element (`self.K2_GetComponentsByClass` "/Script/Engine.ChildActorComponent")
    (bind _asmodule_base (cast `/Game/Timewar/Blueprints/Modules+Equipment/Module_Base` (`ChildActorComponent.ChildActor` _array_element)))
    (if (`|EnumEquality` (`/Game/Timewar/Blueprints/Modules+Equipment/Module_Base.ModuleType` _asmodule_base) "NewEnumerator0")
      (set `/Game/Timewar/Blueprints/Modules+Equipment/Module_Base.(Relative) Formation Slot` (`SceneComponent.RelativeLocation` _array_element) _asmodule_base))
    (`KismetArrayLibrary.Array_Add` (`self.Modules`) _asmodule_base)))