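; RTS squad unit that spawns member actors into ring-based formation slots, arms them with a shared weapon class and can be selected.
; Queued Order objects drive AI movement each Tick, with attack orders closing to weapon range and attack-moves halting while targets are engaged.
; A vision sphere tracks other units in sight.
; Incoming hits wound the living member chosen by distance to the attacking weapon.
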(event `self.ReceiveBeginPlay`
  (`self.CreateHexFormation`)
  (`self.SpawnMembers`)
  (`self.EquipWeaponToAllMembers` (`|GetArrayItem` (`self.WeaponClasses`)))
  (set `self.CurrentOwnership` (`self.OwnedByPlayer`)))

(event `self.VisionSphere.OnComponentBeginOverlap`
  (params (OverlappedComponent :type "PrimitiveComponent Object Reference") (OtherActor :type "Actor Object Reference") (OtherComp :type "PrimitiveComponent Object Reference") (OtherBodyIndex :type Integer) (bFromSweep :type Boolean) (SweepResult :type "HitResult Structure (by ref)"))
  (bind _asunit (cast `/Game/Timewar/Blueprints/Units/Unit` OtherActor))
  (if (not (== self _asunit))
    (`KismetArrayLibrary.Array_Add` (`self.VisibleTargets`) _asunit)))

(event `self.VisionSphere.OnComponentEndOverlap`
  (params (OverlappedComponent :type "PrimitiveComponent Object Reference") (OtherActor :type "Actor Object Reference") (OtherComp :type "PrimitiveComponent Object Reference") (OtherBodyIndex :type Integer))
  (bind _asunit (cast `/Game/Timewar/Blueprints/Units/Unit` OtherActor))
  (`KismetArrayLibrary.Array_RemoveItem` (`self.VisibleTargets`) _asunit))

(event `self.ReceiveTick`
  (params (DeltaSeconds :type "Float (single-precision)"))
  (bind _active_order (`self.Active Order`))
  (`/Engine/EditorBlueprintResources/StandardMacros.IsValid` _active_order
    (:`Is Valid`
      (switch `string` (`/Game/Timewar/Blueprints/Order.ActionToTake` _active_order)
        (:`Attack Enemy Unit`
          (`self.Continuous Move to Unit` 1000.0))
        (:`Move To Location`
          (if (`/Game/Timewar/Blueprints/Order.AttackMove` (`self.Active Order`))
            (if (> (`KismetArrayLibrary.Array_Length` (`self.EngagedTargets`)) 0)
              (`Controller.StopMovement` (`AIBlueprintHelperLibrary.GetAIController` self))
              (else
                (`self.Continuous Move to Location` :!label _label)))
            (else
              (goto _label))))))))

(fn `AddOrder`
  (params (`ShiftHeld?` :type Boolean) (OrderLocation :type "Vector Structure") (OrderActor :type "Actor Object Reference") (`AttackMove?` :type Boolean))
  (if (not `ShiftHeld?`)
    (`KismetArrayLibrary.Array_Clear` (`self.Orders`))
    (set `self.Active Order` null)
    (`Controller.StopMovement` (`AIBlueprintHelperLibrary.GetAIController` self)))
  (bind _returnvalue (`|GenericCreateObject` "/Game/Timewar/Blueprints/Order.Order_C" self))
  (`/Game/Timewar/Blueprints/Order.Construction` _returnvalue OrderLocation OrderActor `AttackMove?`)
  (if (not (> (`KismetArrayLibrary.Array_Length` (`self.Orders`)) 0))
    (set `self.Active Order` _returnvalue))
  (`KismetArrayLibrary.Array_Add` (`self.Orders`) _returnvalue))

(fn `Continuous Move to Location`
  (if (`KismetStringLibrary.EqualEqual_StrStr` (`|GetEnumeratorNameAsString` (`AIController.GetMoveStatus` (`AIBlueprintHelperLibrary.GetAIController` self))) "Idle")
    (if (<= (`KismetMathLibrary.VSize` (- (`/Game/Timewar/Blueprints/Order.LocationOfInterest` (`self.Active Order`)) (`self.K2_GetActorLocation` self))) 500.0)
      (`self.QueueUpNextOrder`)
      (else
        (`NavigationSystem.SimpleMoveToLocation` (`AIBlueprintHelperLibrary.GetAIController` self) (`/Game/Timewar/Blueprints/Order.LocationOfInterest` (`self.Active Order`)))))))

(fn `Continuous Move to Unit`
  (params (Standoff :type "Float (double-precision)"))
  (for _array_element (`self.Equipment`)
    (bind _asweapon (cast `/Game/Timewar/Blueprints/Weapon` _array_element))
    (if (not (>= (`self.DistanceBetweenUnits` (`/Game/Timewar/Blueprints/Order.Unit Of Interest` (`self.Active Order`)) self) (- (`/Game/Timewar/Blueprints/Weapon.MaxRange` _asweapon) 500.0)))
      (`Controller.StopMovement` (`AIBlueprintHelperLibrary.GetAIController` self))
      (return)))
  (`AIController.MoveToActor` (`AIBlueprintHelperLibrary.GetAIController` self) (`/Game/Timewar/Blueprints/Order.Unit Of Interest` (`self.Active Order`)) -1.0 true true true null true)
  (return))

(fn `CreateHexFormation`
  (for _index (range 6)
    (bind _returnvalue (- (* _index 3) 1))
    (for _index_2 (range (+ _returnvalue 1))
      (bind _returnvalue_2 (`KismetMathLibrary.DegreesToRadians` (* _index_2 120.0)))
      (bind _returnvalue_3 (* _index (`self.FormationSpread`)))
      (`KismetArrayLibrary.Array_Add` (`self.FormationSlots`) (`KismetMathLibrary.MakeVector` (* (`KismetMathLibrary.Cos` _returnvalue_2) _returnvalue_3) (* _returnvalue_3 (`KismetMathLibrary.Sin` _returnvalue_2)))))
    (for _index_3 (range (+ _returnvalue 1))
      (bind _returnvalue_4 (`KismetMathLibrary.DegreesToRadians` (* (+ _index_3 60) 120.0)))
      (`KismetArrayLibrary.Array_Add` (`self.FormationSlots`) (`KismetMathLibrary.MakeVector` (* (`KismetMathLibrary.Cos` _returnvalue_4) _returnvalue_3) (* _returnvalue_3 (`KismetMathLibrary.Sin` _returnvalue_4)))))))

(fn `EquipWeaponToAllMembers`
  (params (Class :type "/Game/Timewar/Blueprints/Weapon Class Reference"))
  (for _array_element (`self.Members`)
    (bind _primaryweapon (`/Game/Timewar/Blueprints/Units/UnitMember.PrimaryWeapon` _array_element))
    (`ChildActorComponent.SetChildActorClass` _primaryweapon Class)
    (bind _asweapon (cast `/Game/Timewar/Blueprints/Weapon` (`ChildActorComponent.ChildActor` _primaryweapon)))
    (`KismetArrayLibrary.Array_Clear` (`/Game/Timewar/Blueprints/Weapon.PotentialTargets` _asweapon))
    (set `/Game/Timewar/Blueprints/Weapon.Owning Unit` self _asweapon)
    (`/Game/Timewar/Blueprints/Weapon.Arm Weapon` _asweapon)
    (`KismetArrayLibrary.Array_Add` (`/Game/Timewar/Blueprints/Units/UnitMember.Weapons` _array_element) _asweapon)
    (`KismetArrayLibrary.Array_Add` (`self.Equipment`) _asweapon)
    (`SceneComponent.K2_AttachToComponent` (`/Game/Timewar/Blueprints/Weapon.MaxRangeSphere` _asweapon) (`self.CapsuleComponent`) "None" "SnapToTarget" "SnapToTarget" "SnapToTarget" true)))

(fn `RecieveHit`
  (params (Weapon :type "/Game/Timewar/Blueprints/Weapon Object Reference"))
  (locals (distance :type "Float (double-precision)" :default 1000000000.0) (UnluckyBastard :type "/Game/Timewar/Blueprints/Units/UnitMember Object Reference"))
  (`KismetSystemLibrary.PrintString` "Hit")
  (for _array_element (`self.Members`)
    (bind _returnvalue (`self.GetDistanceTo` _array_element Weapon))
    (if (and (!= (`/Game/Timewar/Blueprints/Units/UnitMember.IsDead` _array_element) true) (< _returnvalue (`local.distance`)))
      (set `local.distance` _returnvalue)
      (set `local.UnluckyBastard` _array_element)))
  (`/Game/Timewar/Blueprints/Units/UnitMember.RecieveWound` (`local.UnluckyBastard`) (`/Game/Timewar/Blueprints/Weapon.Damage` Weapon)))

(fn `SpawnMembers`
  (for (_array_element _array_index) (`self.MemberClasses`)
    (bind _output (`|GetArrayItem` (`self.FormationSlots`) _array_index))
    (bind _returnvalue (`|SpawnActorFromClass` _array_element (`KismetMathLibrary.Conv_VectorToTransform` (+ _output (`self.K2_GetActorLocation` self))) "Undefined" "OverrideRootScale" null null))
    (set `/Game/Timewar/Blueprints/Units/UnitMember.Unit` self _returnvalue)
    (set `/Game/Timewar/Blueprints/Units/UnitMember.AssignedFormationSlot` _output _returnvalue)
    (`KismetArrayLibrary.Array_Add` (`self.Members`) _returnvalue)
    (`/Engine/EditorBlueprintResources/StandardMacros.IncrementInt` 0))
  (return))

(fn `ToggleSelected`
  (params (`Selected?` :type Boolean) (SelectedUnits :type "Array of /Game/Timewar/Blueprints/Units/Unit Object Reference"))
  (if `Selected?`
    (`PrimitiveComponent.SetMaterial` (`self.Cube`) 0 "/Game/StarterContent/Materials/M_AssetPlatform.M_AssetPlatform")
    (set `self.Selected?` true)
    (`KismetArrayLibrary.Array_Add` SelectedUnits self)
    (else
      (`PrimitiveComponent.SetMaterial` (`self.Cube`) 0 "/Game/StarterContent/Materials/M_Tech_Hex_Tile.M_Tech_Hex_Tile")
      (set `self.Selected?` false))))

(fn `UserConstructionScript`)