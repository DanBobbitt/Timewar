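; UnitMember is an AI-controlled member of a Unit that holds a formation slot, takes wounds and can die.
; While alive, it issues a simple move every tick toward its assigned slot offset from the Unit's location.
; Received wounds reduce its wound count, and at zero or below it dies.
; Death plays an animation and smoke effect, stops further move orders and safes each of its weapons.
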(event `self.ReceiveTick`
  (params (DeltaSeconds :type "Float (single-precision)"))
  (if (not (`self.IsDead`))
    (`NavigationSystem.SimpleMoveToLocation` (`AIBlueprintHelperLibrary.GetAIController` self) (+ (`self.AssignedFormationSlot`) (`self.K2_GetActorLocation` (`self.Unit`))))))

(fn `Die`
  (params (DeathType :type String))
  (`SkeletalMeshComponent.PlayAnimation` (`self.Mesh`) "/Game/AnimStarterPack/Death_1.Death_1" false)
  (`GameplayStatics.SpawnEmitterAtLocation` "/Game/StarterContent/Particles/P_Smoke.P_Smoke")
  (set `self.IsDead` true)
  (for _array_element (`self.Weapons`)
    (`/Game/Timewar/Blueprints/Weapon.Safe Weapon` _array_element)))

(fn `RecieveWound`
  (params (`Num Wounds` :type Integer))
  (bind _output_get (set `self.Wounds` (- (`self.Wounds`) `Num Wounds`)))
  (if (<= _output_get 0)
    (`self.Die` "Default")))

(fn `UserConstructionScript`)