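; Base Blueprint for infantry units in Timewar, built from child actor modules.
; The construction script collects Module_Base child actors into a Modules array, storing each component's relative location as the formation slot for one module type.
; A Unit Death graph unregisters the unit from the game state, removes it from the player's selection, gives a set of actors a brief lifespan and destroys itself.
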(event `self.ReceiveBeginPlay`)

(fn `UserConstructionScript`
  (for _array_element (`self.K2_GetComponentsByClass` "/Script/Engine.ChildActorComponent")
    (bind _asmodule_base (cast `/Game/Timewar/Blueprints/Modules+Equipment/Module_Base` (`ChildActorComponent.ChildActor` _array_element)))
    (if (`|EnumEquality` (`/Game/Timewar/Blueprints/Modules+Equipment/Module_Base.ModuleType` _asmodule_base) "NewEnumerator0")
      (set `/Game/Timewar/Blueprints/Modules+Equipment/Module_Base.(Relative) Formation Slot` (`SceneComponent.RelativeLocation` _array_element) _asmodule_base))
    (`KismetArrayLibrary.Array_Add` (`self.Modules`) _asmodule_base)))