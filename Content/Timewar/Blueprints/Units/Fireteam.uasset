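; Fireteam is a member of a Unit that follows it in loose formation and can be killed by wounds.
; While alive, it moves every tick toward the Unit's location plus an offset, which each received order re-randomizes around its assigned relative position.
; Wounds count down to Die, which spawns sparks, flags it dead, then safes each weapon and removes it from the Unit's members inside the same loop.
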(event `self.ReceiveTick`
  (params (DeltaSeconds :type "Float (single-precision)"))
  (if (not (`self.IsDead`))
    (`NavigationSystem.SimpleMoveToLocation` (`AIBlueprintHelperLibrary.GetAIController` self) (+ (`self.RandomizedPosition`) (`self.K2_GetActorLocation` (`self.Unit`))))))

(event `Recieve Order`
  (bind (_positionrelativetounit_x _positionrelativetounit_y _positionrelativetounit_z) (`KismetMathLibrary.BreakVector` (`self.PositionRelativeToUnit`)))
  (set `self.RandomizedPosition` (`KismetMathLibrary.MakeVector` (+ (`KismetMathLibrary.RandomFloatInRange` -400.0 400.0) _positionrelativetounit_x) (+ (`KismetMathLibrary.RandomFloatInRange` -400.0 400.0) _positionrelativetounit_y) _positionrelativetounit_z)))

(fn `Die`
  (params (DeathType :type String))
  (bind (_returnvalue_location _returnvalue_rotation) (`KismetMathLibrary.BreakTransform` (`SceneComponent.K2_GetComponentToWorld` (`self.Fireteam`))))
  (`GameplayStatics.SpawnEmitterAtLocation` "/Game/StarterContent/Particles/P_Sparks.P_Sparks" _returnvalue_location _returnvalue_rotation)
  (set `self.IsDead` true)
  (for _array_element (`self.Weapons`)
    (`/Game/Timewar/Blueprints/Weapon.Safe Weapon` _array_element)
    (`KismetArrayLibrary.Array_RemoveItem` (`/Game/Timewar/Blueprints/Units/Unit.Members` (`self.Unit`)) self)))

(fn `RecieveWound`
  (params (`Num Wounds` :type Integer))
  (bind _output_get (set `self.Wounds` (- (`self.Wounds`) `Num Wounds`)))
  (if (<= _output_get 0)
    (`self.Die` "Default")))

(fn `UserConstructionScript`)