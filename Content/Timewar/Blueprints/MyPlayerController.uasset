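; Player controller for RTS-style unit selection and orders, which also forwards commander spawn requests to MyTrueGameMode.
; BoxSelect gathers Units inside a HUD rectangle into CurrentlySelectedUnits, clearing the previous selection unless Left Shift is held.
; Right-click traces from the cursor on the Camera channel, with debug drawing on, and gives each selected unit an order at the hit location, flagged by Shift and A for attack-move.
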(event `ROS_SetPlayerToSpawn`
  (params (Commander :type "Pawn Class Reference") (SpawnTransform :type "Transform Structure") (PlayerController :type "PlayerController Object Reference"))
  (bind _asmy_true_game_mode (cast `/Game/Timewar/Blueprints/MyTrueGameMode` (`GameplayStatics.GetGameMode`)))
  (`/Game/Timewar/Blueprints/MyTrueGameMode.Spawn Player Character` _asmy_true_game_mode Commander SpawnTransform PlayerController))

(event `Box Select`
  (params (TopLeftRectCorner :type "Vector2D Structure") (BottomRightRectCorner :type "Vector2D Structure"))
  (if (`self.IsInputKeyDown` "LeftShift")
    (for _array_element (`HUD.GetActorsInSelectionRectangle` (`self.GetHUD`) "/Game/Timewar/Blueprints/Units/Unit.Unit_C" TopLeftRectCorner BottomRightRectCorner false false) :!label _label
      (bind _asunit (cast `/Game/Timewar/Blueprints/Units/Unit` _array_element))
      (`KismetArrayLibrary.Array_Add` (`self.CurrentlySelectedUnits`) _asunit)
      (`/Game/Timewar/Blueprints/Units/Unit.Selected` _asunit))
    (else
      (`|ExecutionSequence`
        (:`then_0`
          (for _array_element_2 (`self.CurrentlySelectedUnits`)
            (`/Game/Timewar/Blueprints/Units/Unit.Deselected` _array_element_2))
          (`KismetArrayLibrary.Array_Clear` (`self.CurrentlySelectedUnits`)))
        (:`then_1`
          (goto _label))))))

(event `Key|RightMouseButton`
  (params (Key :type "Key Structure"))
  (bind (_worldlocation _worlddirection) (`self.DeprojectMousePositionToWorld`))
  (:`Pressed`
    (bind (_outhit _returnvalue) (`KismetSystemLibrary.LineTraceSingle` :`Start` _worldlocation :`End` (+ (* _worlddirection 1000000.0) _worldlocation) :`TraceChannel` "TraceTypeQuery2" :`DrawDebugType` "ForDuration"))
    (if _returnvalue
      (for _array_element (`self.CurrentlySelectedUnits`)
        (`/Game/Timewar/Blueprints/Units/Unit.AddOrder` _array_element (`self.IsInputKeyDown` "LeftShift") (`.Location` (`GameplayStatics.BreakHitResult` _outhit)) null (`self.IsInputKeyDown` "A"))))))

(fn `UserConstructionScript`)