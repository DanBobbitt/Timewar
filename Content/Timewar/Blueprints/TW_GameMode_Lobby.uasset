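; Lobby game mode for Timewar that tracks connected players and moves the match into setup and game phases.
; On login it registers and initializes each controller, then pushes player lists, selected armies, counts and map settings to all controllers.
; Refreshing player info also sets CanWeStart based on every player having a named army.
; Phase events notify controllers and update GameStatus, with game start also executing active units' orders inside the per-controller loop.
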(event `self.K2_PostLogin`
  (params (NewPlayer :type "PlayerController Object Reference"))
  (bind _astw_player_controller_lobby (cast `/Game/Timewar/Blueprints/TW_PlayerController_Lobby` NewPlayer :!pure true))
  ;[1 1 1] When a client logs in
  (`/Engine/EditorBlueprintResources/ActorMacros.Switch Has Authority`
    (:`Authority`
      (`KismetArrayLibrary.Array_Add` (`self.AllPlayerControllers`) _astw_player_controller_lobby)
      (`/Game/Timewar/Blueprints/TW_PlayerController_Lobby.Post Login Server` _astw_player_controller_lobby)
      (`/Game/Timewar/Blueprints/TW_PlayerController_Lobby.Post Login Client` _astw_player_controller_lobby (`self.ServerName`))
      (`self.UpdateAllPlayerInfo`)
      (`/Game/Timewar/Blueprints/TW_PlayerController_Lobby.UpdateMatchSettings` _astw_player_controller_lobby (`self.GamemodeMapImage`) (`self.GamemodeMapName`) (`self.GamemodeMapTime`)))))

(event `UpdateAllPlayerInfo`
  (bind _allplayercontrollers (`self.AllPlayerControllers`))
  ;[1 1 1] Updates All Player's Lobby Information
  (bind _output_get (set `self.NumPlayers` (`KismetArrayLibrary.Array_Length` (`self.AllPlayerControllers`))))
  (if (> _output_get 0)
    (`KismetArrayLibrary.Array_Clear` (`self.ConnectedPlayerInfos`))
    (`KismetArrayLibrary.Array_Clear` (`self.ConnectedPlayerArmies`))
    (for _array_element _allplayercontrollers
      (bind _astw_player_controller_lobby (cast `/Game/Timewar/Blueprints/TW_PlayerController_Lobby` _array_element))
      (`KismetArrayLibrary.Array_Add` (`self.ConnectedPlayerInfos`) (`/Game/Timewar/Blueprints/TW_PlayerController_Lobby.PlayerInfo` _astw_player_controller_lobby))
      (`KismetArrayLibrary.Array_Add` (`self.ConnectedPlayerArmies`) (`/Game/Timewar/Blueprints/TW_PlayerController_Lobby.SelectedArmy` _astw_player_controller_lobby))
      (`/Game/Timewar/Blueprints/TW_PlayerController_Lobby.UpdateNumberOfPlayers` _astw_player_controller_lobby (`self.NumPlayers`) (`self.MaxPlayers`)))
    (for _array_element_2 _allplayercontrollers
      (bind _astw_player_controller_lobby_2 (cast `/Game/Timewar/Blueprints/TW_PlayerController_Lobby` _array_element_2))
      (`/Game/Timewar/Blueprints/TW_PlayerController_Lobby.UpdatePlayerList` _astw_player_controller_lobby_2 (`self.ConnectedPlayerInfos`) (`self.ConnectedPlayerArmies`)))
    (for _array_element_3 (`self.ConnectedPlayerArmies`) :!label _label
      (if (`KismetTextLibrary.TextIsEmpty` (`.ArmyName_4_F57878CB4372AE4D42EE2398FEC5274B` (break `/Game/Timewar/Structs/Army` _array_element_3)))
        (set `self.CanWeStart?` false)
        (`self.break`)
        (else
          (set `self.CanWeStart?` true))))
    (else
      (`KismetSystemLibrary.PrintString` "EverybodyUpdate: Number of players = 0!"))))

(event `Break`
  ;[1 1 1] Updates All Player's Lobby Information
  (goto _label :!via `Break`))

(event `ServerUpdateGameSettings`
  (params (MapImage :type "Texture2D Object Reference") (MapName :type Text) (MapTime :type Text))
  ;[1 1 1] Server made changes, update our lobby info for clients
  (set `self.GamemodeMapImage` MapImage)
  (set `self.GamemodeMapName` MapName)
  (set `self.GamemodeMapTime` MapTime)
  (for _array_element (`self.AllPlayerControllers`)
    (bind _astw_player_controller_lobby (cast `/Game/Timewar/Blueprints/TW_PlayerController_Lobby` _array_element))
    (`/Game/Timewar/Blueprints/TW_PlayerController_Lobby.UpdateMatchSettings` _astw_player_controller_lobby (`self.GamemodeMapImage`) (`self.GamemodeMapName`) (`self.GamemodeMapTime`))))

(event `Begin Setup Phase`
  (for _array_element (`self.AllPlayerControllers`)
    (bind _astw_player_controller_lobby (cast `/Game/Timewar/Blueprints/TW_PlayerController_Lobby` _array_element))
    (`/Game/Timewar/Blueprints/TW_PlayerController_Lobby.Begin Setup Phase` _astw_player_controller_lobby)
    (set `self.GameStatus` "NewEnumerator2")))

(event `Begin Game`
  (for _array_element (`self.AllPlayerControllers`)
    (bind _astw_player_controller_lobby (cast `/Game/Timewar/Blueprints/TW_PlayerController_Lobby` _array_element))
    (`/Game/Timewar/Blueprints/TW_PlayerController_Lobby.Begin Game Phase` _astw_player_controller_lobby)
    (set `self.GameStatus` "NewEnumerator3")
    (for _array_element_2 (`/Game/Timewar/Blueprints/TW_GameState.ActiveUnits` (cast `/Game/Timewar/Blueprints/TW_GameState` (`GameplayStatics.GetGameState`) :!pure true))
      (`/Game/Timewar/Blueprints/Units/Unit_Base.ExecuteOrder` _array_element_2))))

(fn `UserConstructionScript`)