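; Player-possessed RTS commander pawn that drives the camera and issues commands to units.
; Camera macros handle axis movement, Alt-drag rotation, middle-mouse panning and screen-edge scrolling, with gates routing mouse input between modes.
; Wheel zoom uses the deprojected cursor position to shift the camera rig along the mouse ray.
; Cursor line traces drive click and Shift selection of Units, then right-click orders with Shift and A (attack-move) modifiers.
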(event `self.ReceivePossessed`
  (params (NewController :type "Controller Object Reference"))
  (bind _asmy_player_controller (cast `/Game/Timewar/Blueprints/MyPlayerController` NewController))
  (set `self.OwningController` _asmy_player_controller))

(event `self.ReceiveBeginPlay`
  (set `PlayerController.bShowMouseCursor` true (`GameplayStatics.GetPlayerController` 0)))

(event `self.ReceiveUnpossessed`
  (params (OldController :type "Controller Object Reference"))
  (set `self.OwningController` null))

(event `InputAxis|MoveForward`
  (params (AxisValue :type "Float (single-precision)"))
  ;[1 1 1] Camera Movement  + Zoom
  (`self.Camera Move Macro` AxisValue (stale `InputAxis|MoveRight` AxisValue) :!label _label))

(event `Key|MouseScrollUp`
  (params (Key :type "Key Structure"))
  ;[1 1 1] Camera Movement  + Zoom
  (:`Pressed`
    (`self.Camera Zoom Macro` :!label _label_2)))

(event `Key|MouseScrollDown`
  (params (Key :type "Key Structure"))
  ;[1 1 1] Camera Movement  + Zoom
  (:`Pressed`
    (goto _label_2 :!via `Zoom Out`)))

(event `InputAxis|MoveRight`
  (params (AxisValue :type "Float (single-precision)"))
  ;[1 1 1] Camera Movement  + Zoom
  (goto _label :!via `Left and Right`))

(event `Key|LeftAlt`
  (params (Key :type "Key Structure"))
  ;[1 1 1] Rotation, Panning or Screen Edge
  (:`Pressed`
    (set `self.Camera Rotating` true)
    (`|ExecutionSequence`
      (:`then_0`
        (goto _label_3 :!via `Open`))
      (:`then_1`
        (goto _label_8 :!via `Open`))))
  (:`Released`
    (set `self.Camera Rotating` false)
    (`|ExecutionSequence`
      (:`then_0`
        (goto _label_3 :!via `Close`))
      (:`then_1`
        (goto _label_8 :!via `Close`)))))

(event `InputAxisKey|MouseX`
  (params (AxisValue :type "Float (single-precision)"))
  ;[1 1 1] Rotation, Panning or Screen Edge
  (if (xor (`self.Camera Rotating`) (`self.Camera Panning`))
    (if (`self.Camera Rotating`)
      (`/Engine/EditorBlueprintResources/StandardMacros.Gate` true :!label _label_3
        (:`Exit`
          (`self.Camera Rotate Macro` AxisValue (stale `InputAxisKey|MouseY` AxisValue) :!label _label_4)))
      (else
        (`/Engine/EditorBlueprintResources/StandardMacros.Gate` true :!label _label_5
          (:`Exit`
            (`self.Camera Pan Macro` AxisValue (stale `InputAxisKey|MouseY` AxisValue) :!label _label_6)))))
    (else
      (`self.Camera Screenedge Macro` :!label _label_7))))

(event `InputAxisKey|MouseY`
  (params (AxisValue :type "Float (single-precision)"))
  ;[1 1 1] Rotation, Panning or Screen Edge
  (if (xor (`self.Camera Rotating`) (`self.Camera Panning`))
    (if (`self.Camera Rotating`)
      (`/Engine/EditorBlueprintResources/StandardMacros.Gate` true :!label _label_8
        (:`Exit`
          (goto _label_4 :!via `Mouse LeftRight`)))
      (else
        (`/Engine/EditorBlueprintResources/StandardMacros.Gate` true :!label _label_9
          (:`Exit`
            (goto _label_6 :!via `MouseY`)))))
    (else
      (goto _label_7 :!via `ForwardAndBack`))))

(event `Key|MiddleMouseButton`
  (params (Key :type "Key Structure"))
  ;[1 1 1] Rotation, Panning or Screen Edge
  (:`Pressed`
    (set `self.Camera Panning` true)
    (`|ExecutionSequence`
      (:`then_0`
        (goto _label_5 :!via `Open`))
      (:`then_1`
        (goto _label_9 :!via `Open`))))
  (:`Released`
    (set `self.Camera Panning` false)
    (`|ExecutionSequence`
      (:`then_0`
        (goto _label_5 :!via `Close`))
      (:`then_1`
        (goto _label_9 :!via `Close`)))))

(event `Key|LeftShift`
  (params (Key :type "Key Structure"))
  ;[1 1 1] Unit Selection
  (:`Pressed`
    (set `self.ShiftHeld` true))
  (:`Released`
    (set `self.ShiftHeld` false)))

(event `Key|LeftMouseButton`
  (params (Key :type "Key Structure"))
  (bind _selectedunits (`self.SelectedUnits`))
  (bind _selectedunits_2 (`self.SelectedUnits`))
  ;[1 1 1] Unit Selection
  (:`Released`
    (bind _outhit (`self.LineTraceMousePosition`))
    (`KismetSystemLibrary.PrintString` (`KismetSystemLibrary.GetDisplayName` (`.HitActor` (`GameplayStatics.BreakHitResult` _outhit))))
    (bind _asunit (cast `/Game/Timewar/Blueprints/Units/Unit` (`.HitActor` (`GameplayStatics.BreakHitResult` _outhit)))
      (:`then`
        (if (`self.ShiftHeld`)
          (`/Game/Timewar/Blueprints/Units/Unit.ToggleSelected` _asunit true (`self.SelectedUnits`))
          (else
            (bind _outactors (`GameplayStatics.GetAllActorsOfClass` "/Game/Timewar/Blueprints/Units/Unit.Unit_C"))
            (for _array_element _outactors
              (`/Game/Timewar/Blueprints/Units/Unit.ToggleSelected` _array_element false _selectedunits_2))
            (`KismetArrayLibrary.Array_Clear` _selectedunits_2)
            (`/Game/Timewar/Blueprints/Units/Unit.ToggleSelected` _asunit true (`self.SelectedUnits`)))))
      (:`CastFailed`
        (bind _outactors_2 (`GameplayStatics.GetAllActorsOfClass` "/Game/Timewar/Blueprints/Units/Unit.Unit_C"))
        (for _array_element_2 _outactors_2
          (`/Game/Timewar/Blueprints/Units/Unit.ToggleSelected` _array_element_2 false _selectedunits))
        (`KismetArrayLibrary.Array_Clear` _selectedunits)))))

(event `Key|A`
  (params (Key :type "Key Structure"))
  ;[1 1 1] Unit Selection
  (:`Pressed`
    (set `self.AHeld` true))
  (:`Released`
    (set `self.AHeld` false)))

(event `Key|RightMouseButton`
  (params (Key :type "Key Structure"))
  (:`Released`
    (bind (_outhit _hit_) (`self.LineTraceMousePosition`))
    (if _hit_
      (for _array_element (`self.SelectedUnits`)
        (`/Game/Timewar/Blueprints/Units/Unit.AddOrder` _array_element (`self.ShiftHeld`) (`.Location` (`GameplayStatics.BreakHitResult` _outhit)) (`.HitActor` (`GameplayStatics.BreakHitResult` _outhit)) (`self.AHeld`))))))

(fn `LineTraceMousePosition`
  (returns (OutHit :type "HitResult Structure") (`Hit?` :type Boolean))
  (bind _owningcontroller (`self.OwningController`))
  (bind (_worldlocation _worlddirection) (`PlayerController.DeprojectMousePositionToWorld` _owningcontroller))
  (if (`KismetSystemLibrary.IsValid` _owningcontroller)
    (bind (_outhit _returnvalue) (`KismetSystemLibrary.LineTraceSingle` _worldlocation (+ (* _worlddirection 100000.0) _worldlocation) "TraceTypeQuery1"))
    (return _outhit _returnvalue)
    (else
      (return (struct) false))))

(fn `UserConstructionScript`)